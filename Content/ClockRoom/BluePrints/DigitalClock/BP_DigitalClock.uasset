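; Digital clock actor that shows the current system time as text in HH:MM:SS format.
; Every Tick it reads hour, minute and second from Now and pads each below ten with a leading zero.
; The joined string goes straight to the Digits text component, while the construction script does nothing.
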(event EventBeginPlay)

(event Collision|EventActorBeginOverlap
  (params (OtherActor :type Actor%20Object%20Reference)))

(event EventTick
  (params (DeltaSeconds :type Float%20%28single-precision%29))
  (bind _returnvalue (Math|DateTime|Now))
  (bind _returnvalue_2 (Class|KismetMathLibrary|GetHour _returnvalue))
  (bind _returnvalue_3 (Class|KismetMathLibrary|GetMinute _returnvalue))
  (bind _returnvalue_4 (Class|KismetMathLibrary|GetSecond _returnvalue))
  (bind _returnvalue_5 (Utilities|String|ToString(Integer) _returnvalue_2))
  (bind _returnvalue_6 (Utilities|String|ToString(Integer) _returnvalue_3))
  (bind _returnvalue_7 (Utilities|String|ToString(Integer) _returnvalue_4))
  ;[1 1 1] Digital clock with format 00:00:00
  (Rendering|Components|TextRender|SetText (Variables|Default|GetDigits) (Utilities|Text|ToText(String) (Utilities|String|Append (select (> _returnvalue_2 9) _returnvalue_5 (Utilities|String|Append "0" _returnvalue_5)) ":" (select (> _returnvalue_3 9) _returnvalue_6 (Utilities|String|Append "0" _returnvalue_6)) ":" (select (> _returnvalue_4 9) _returnvalue_7 (Utilities|String|Append "0" _returnvalue_7))))))

(fn ConstructionScript)