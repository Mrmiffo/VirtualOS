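; A grabbable VR lever that acts as a program shortcut with a name and icon, starting and closing its assigned program.
; While grabbed, Tick rotates the handle with the hand's roll, which triggers TurnOn or TurnOff near either extreme; release snaps it to neutral.
; TurnOn spawns one program instance where the VrOsPawn looks and passes it a test startup path, TurnOff destroys it, and both recolor the handle's dynamic material.
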(event EventBeginPlay
  ;[1 1 1] Set the handle material to a material that can change glow
  (bind _returnvalue (Rendering|Material|CreateDynamicMaterialInstance "/Game/MenuThings/changingMaterial.changingMaterial" :!class /Script/Engine.KismetMaterialLibrary))
  (bind _output_get (Variables|Default|SethandleMaterial _returnvalue))
  (Rendering|Material|SetMaterial (Variables|Default|Gethandle) 0 _output_get)
  (Variables|Default|Setstartcolor "(R=0.200891,G=0.900000,B=0.175500,A=1.000000)")
  (Variables|Default|Setstandbycolor "(R=0.665000,G=0.665000,B=0.665000,A=1.000000)")
  (Variables|Default|Setshutdowncolor "(R=0.625000,G=0.315251,B=0.300000,A=1.000000)")
  (CallFunction|SetHandleColor (Variables|Default|Getshutdowncolor)))

(event EventDrop
  ;[1 0.02672 0.1164] Set is not grabbedf
  (Variables|Default|SetbeingGrabbed false))

(event EventTick
  (params (DeltaSeconds :type Float%20%28single-precision%29))
  ;[1 1 1] each tick, check if being grabbed
  (if (Variables|Default|GetbeingGrabbed)
    ;[1 1 1] make the handle follow the hands rotation
    (bind _handrotation (CallFunction|GetHandRotation))
    (Transformation|SetRelativeRotation (Variables|Default|GetScene) (Math|Rotator|MakeRotator (* -1 _handrotation) 0.0 0.0) false false)
    (Utilities|FlowControl|Sequence
      (:then_0
        ;[1 1 1] turn off if handle moved to off
        (if (Math|Float|InRange(Float) _handrotation -9e+01 -6e+01)
          (CallFunction|TurnOff)))
      (:then_1
        ;[1 1 1] turn on if handle moved to on
        (if (Math|Float|InRange(Float) _handrotation 6e+01 9e+01)
          (CallFunction|Turnon))))
    (else
      (Transformation|SetRelativeRotation (Variables|Default|GetScene) "0, 0, 0" false false))))

(event EventEndGrab
  ;[1 0.02672 0.1164] Set is not grabbedf
  (Variables|Default|SetbeingGrabbed false))

(event EventStartGrab
  (params (GrabbingController :type Motion%20Controller%20Component%20Object%20Reference))
  ;[1 1 1] set is grabbed
  (Variables|Default|SetGrabbingHand GrabbingController)
  (Variables|Default|SetbeingGrabbed true))

(fn ConstructionScript)

(fn InitializeButton
  (params (programToStart :type Actor%20Class%20Reference) (shortcutName :type Text) (vrOsPawn :type Virtual%20OS%20Pawn%20Object%20Reference) (shortcutIcon :type Texture%20Object%20Reference))
  (Variables|Default|SetprogramToStart programToStart)
  (Rendering|Components|TextRender|SetText (Variables|Default|GetshortcutText) shortcutName)
  (Variables|Default|SetvrOsPawn vrOsPawn)
  (Development|PrintString "lever aknowledged vrospawn" true true "(R=0.000000,G=0.660000,B=1.000000,A=1.000000)" 1e+03)
  (bind _returnvalue (Rendering|Material|CreateDynamicMaterialInstance "/Game/MenuThings/shortcutTextures/iconMaterial.iconMaterial" :!class /Script/Engine.KismetMaterialLibrary))
  (Rendering|Material|SetTextureParameterValue _returnvalue "textureParam" shortcutIcon)
  (Rendering|Material|SetMaterial (Variables|Default|GetStaticMesh) 0 _returnvalue))

(fn SetHandleColor
  (params (Color :type Linear%20Color%20Structure))
  (Rendering|Material|SetVectorParameterValue (Variables|Default|GethandleMaterial) "color" Color :!class /Script/Engine.MaterialInstanceDynamic))

(fn Turnon
  ;[1 1 1] try to turn on
  (CallFunction|SetHandleColor (Variables|Default|Getstartcolor))
  ;[1 1 1] dont start another  if program already started
  (if (not (Utilities|IsValid (Variables|Default|GetstartedProgram)))
    ;[1 1 1] Has the button been assigned a program?
    (if (Utilities|IsValidClass (Variables|Default|GetprogramToStart))
      ;[1 1 1] start the program its been told to start
      (bind _pointlookedat (Default|GetLookingat (Variables|Default|GetvrOsPawn) 1e+02))
      (bind _returnvalue (Game|SpawnActorfromClass (Variables|Default|GetprogramToStart) _pointlookedat "Undefined" 0 0))
      (bind _output_get (Variables|Default|SetstartedProgram _returnvalue))
      ;[1 0 0] SUCH HARD CODE FOR TEST 2
      (bind _asprogram (Utilities|Casting|CastToprogram _output_get))
      (Default|OnStartup _asprogram (Class|FileSystemBPLibrary|GetContainingFolderPath (Class|FileSystemBPLibrary|GetPathtoUserDir)))
      (else
        (Development|PrintString "Handle has not been assigned a program to start!" true true "(R=1.000000,G=0.076668,B=0.000000,A=1.000000)" 1e+01)))))

(fn TurnOff
  (CallFunction|SetHandleColor (Variables|Default|Getshutdowncolor))
  ;[1 1 1] is a program running?
  (if (Utilities|IsValid (Variables|Default|GetstartedProgram))
    ;[1 1 1] close program
    (Actor|DestroyActor (Variables|Default|GetstartedProgram))))

(fn GetHandRotation
  (return (.Roll (Math|Rotator|BreakRotator (Transformation|GetWorldRotation (Variables|Default|GetGrabbingHand))))))