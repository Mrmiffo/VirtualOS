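; Start menu actor that spawns a row of program shortcut buttons in the world when play begins.
; BeginPlay adds six hardcoded entries, a mix of TraditionalClock and ClockText, through AddStartButton.
; AddStartButton spawns a ProgramButton actor at the ButtonRowStart component, offset along world Y by the running program count, then tells it what to start.
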(event EventBeginPlay
  (CallFunction|AddStartButton "/Game/Test/JohanFolder/Blueprints/traditionalClock/TraditionalClock.TraditionalClock_C")
  (CallFunction|AddStartButton "/Game/Test/JohanFolder/Blueprints/ClockText.ClockText_C")
  (CallFunction|AddStartButton "/Game/Test/JohanFolder/Blueprints/traditionalClock/TraditionalClock.TraditionalClock_C")
  (CallFunction|AddStartButton "/Game/Test/JohanFolder/Blueprints/traditionalClock/TraditionalClock.TraditionalClock_C")
  (CallFunction|AddStartButton "/Game/Test/JohanFolder/Blueprints/traditionalClock/TraditionalClock.TraditionalClock_C")
  (CallFunction|AddStartButton "/Game/Test/JohanFolder/Blueprints/ClockText.ClockText_C"))

(fn ConstructionScript)

(fn AddStartButton
  (params (NewParam :type Actor%20Class%20Reference))
  (bind _buttonrowstart (Variables|Default|GetbuttonRowStart))
  (bind _returnvalue (Transformation|GetWorldLocation _buttonrowstart))
  (bind (_x _y _z) (Math|Vector|BreakVector _returnvalue))
  (bind _returnvalue_2 (Game|SpawnActorfromClass "/Game/Test/JohanFolder/Blueprints/Menu/programButton.programButton_C" (Math|Transform|MakeTransform (Math|Vector|MakeVector _x (+ _y (Math|Conversions|ToFloat(Integer) (* (Variables|Default|GetamountOfPrograms) 40))) _z)) "Undefined" 0 0))
  ;[1 1 1] set the button shortcut
  (Default|SetWhattoStart _returnvalue_2 NewParam)
  ;[1 1 1] remember how many buttons there re
  (Math|Integer|IncrementInt (Variables|Default|GetamountOfPrograms)))