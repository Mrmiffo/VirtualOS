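; Menu button actor that launches a program actor when something overlaps it or the H key is pressed.
; If not already open, it spawns the configurable WhatToStart class at StartLocation and keeps a reference to it.
; It also spawns a CloseButton at CloseLocation, handing it the program and itself.
; ProgramClosed clears the Open flag so the program can launch again.
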(event EventBeginPlay
  ;[1 1 1] should listen for input
  (Input|EnableInput (Game|GetPlayerController 0))
  ;[1 1 1] default closed
  (Variables|Default|Setopen false))

(event Collision|EventActorBeginOverlap
  (params (OtherActor :type Actor%20Object%20Reference))
  (Development|PrintString "Button collide!!!")
  ;[1 1 1] create program
  ;;[1 1 1] if not already open
  (if (not (Variables|Default|Getopen))
    ;;[1 1 1] start program
    (bind _returnvalue (Game|SpawnActorfromClass (Variables|Default|GetwhatToStart) (Math|Transform|MakeTransform (Transformation|GetWorldLocation (Variables|Default|GetstartLocation)) (Transformation|GetWorldRotation (Variables|Default|GetstartLocation)) "1.000000,1,1") "Undefined" 0 0))
    ;[1 1 1] remember is open
    (Variables|Default|Setopen true)
    ;[1 1 1] remember ref to started program
    (Variables|Default|SetOpenedActor _returnvalue)
    ;[1 1 1] Create close button
    (bind _returnvalue_2 (Game|SpawnActorfromClass "/Game/Test/JohanFolder/Blueprints/Menu/closeButton.closeButton_C" (Math|Transform|MakeTransform (Transformation|GetWorldLocation (Variables|Default|GetcloseLocation))) "Undefined" 0 0))
    (Default|SetProgramtoClose _returnvalue_2 (Variables|Default|GetopenedActor) self)))

(event Input|KeyboardEvents|H
  (params (Key :type Key%20Structure :default "AnyKey"))
  ;[1 1 1] create program
  (:Pressed
    ;;[1 1 1] if not already open
    (if (not (Variables|Default|Getopen))
      ;;[1 1 1] start program
      (bind _returnvalue (Game|SpawnActorfromClass (Variables|Default|GetwhatToStart) (Math|Transform|MakeTransform (Transformation|GetWorldLocation (Variables|Default|GetstartLocation)) (Transformation|GetWorldRotation (Variables|Default|GetstartLocation)) "1.000000,1,1") "Undefined" 0 0))
      ;[1 1 1] remember is open
      (Variables|Default|Setopen true)
      ;[1 1 1] remember ref to started program
      (Variables|Default|SetOpenedActor _returnvalue)
      ;[1 1 1] Create close button
      (bind _returnvalue_2 (Game|SpawnActorfromClass "/Game/Test/JohanFolder/Blueprints/Menu/closeButton.closeButton_C" (Math|Transform|MakeTransform (Transformation|GetWorldLocation (Variables|Default|GetcloseLocation))) "Undefined" 0 0))
      (Default|SetProgramtoClose _returnvalue_2 (Variables|Default|GetopenedActor) self))))

(fn ConstructionScript)

(fn SetWhattoStart
  (params (inputClass :type Actor%20Class%20Reference))
  (Variables|Default|SetwhatToStart inputClass))

(fn ProgramClosed
  (Variables|Default|Setopen false))