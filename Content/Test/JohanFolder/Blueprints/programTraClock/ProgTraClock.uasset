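; An analog clock actor that shows the current system time with rotating hour, minute and second hands.
; BeginPlay enables input, then a one-second Delay loop sets each hand's pitch from Now(), with the hour hand stepping in whole hours.
; Y toggles an edit mode that shows a cube, in which T and R uniformly grow or shrink the actor within size limits, printing an error otherwise.
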(event EventBeginPlay
  (bind _returnvalue (Math|DateTime|Now))
  ;[1 1 1] Digital clock text, that updates every second.
  (Input|EnableInput (Game|GetPlayerController 0))
  (Utilities|FlowControl|Delay 1.0 :!label _label)
  ;;[1 1 1] second
  (Transformation|SetRelativeRotation (Variables|Default|GetSecondHandScene) (Math|Rotator|MakeRotator 0.0 (+ (* (Math|Conversions|ToFloat(Integer) (Class|KismetMathLibrary|GetSecond _returnvalue)) -6.0) 1.8e+02) 0.0) false false)
  ;;[1 1 1] minute
  (Transformation|SetRelativeRotation (Variables|Default|Getminutehandscene) (Math|Rotator|MakeRotator 0.0 (+ (* (Class|KismetMathLibrary|GetMinute _returnvalue) -6.0) 1.8e+02) 0.0) false false)
  (Transformation|SetRelativeRotation (Variables|Default|GethourHandScene) (Math|Rotator|MakeRotator 0.0 (+ (* (Math|Integer|%(Integer) (Class|KismetMathLibrary|GetHour _returnvalue) 12) -3e+01) 1.8e+02) 0.0) false false)
  (goto _label))

(event Input|KeyboardEvents|T
  (params (Key :type Key%20Structure :default "AnyKey"))
  ;[1 1 1] make bigger
  (:Pressed
    ;;[1 1 1] if is editing
    (if (Variables|Default|GetinEditMode)
      ;;[1 1 1] can i become bigger
      (if (< (+ (Variables|Default|Getsize) 0.1) 1e+03)
        ;;[1 1 1] remember new size
        (bind _output_get (Variables|Default|Setsize (+ (Variables|Default|Getsize) 0.1)))
        ;;[1 1 1] scale to new actor size
        (Transformation|SetActorRelativeScale3D (Math|Vector|MakeVector _output_get _output_get _output_get))
        (else
          ;;[1 1 1] error size
          (Development|PrintString "this is just way too big"))))))

(event Input|KeyboardEvents|R
  (params (Key :type Key%20Structure :default "AnyKey"))
  ;[1 1 1] make smaller
  ;;[1 1 1] if is in edit mode
  (:Pressed
    (if (Variables|Default|GetinEditMode)
      ;;[1 1 1] can it become smaller?
      (if (> (- (Variables|Default|Getsize) 0.1) 0.0)
        ;;[1 1 1] remember new size
        (bind _output_get (Variables|Default|Setsize (- (Variables|Default|Getsize) 0.1)))
        ;;[1 1 1] scale the actor to the size
        (Transformation|SetActorRelativeScale3D (Math|Vector|MakeVector _output_get _output_get _output_get))
        (else
          ;;[1 1 1] error print if size 0
          (Development|PrintString "cannot have negative or 0 size"))))))

(event Input|KeyboardEvents|Y
  (params (Key :type Key%20Structure :default "AnyKey"))
  ;[1 1 1] toggle edit mode
  (:Pressed
    (bind _output_get (Variables|Default|SetinEditMode (not (Variables|Default|GetinEditMode))))
    (Rendering|SetVisibility (Variables|Default|GetCube) _output_get false)))

(fn ConstructionScript)