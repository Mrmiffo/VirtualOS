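; ClockText is a test Blueprint that shows a digital clock on a TextRender component, updated every second.
; From BeginPlay, a one-second Delay loops back on itself, so the first update comes after one second.
; Each pass rebuilds the text from the current system hour, minute and second, joined by a Seperator variable without zero-padding.
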(event EventBeginPlay
  (bind _returnvalue (Math|DateTime|Now))
  ;[1 1 1] Digital clock text, that updates every second.
  (Utilities|FlowControl|Delay 1.0 :!label _label)
  (Rendering|Components|TextRender|SetText (Variables|Default|GetTextRender) (Utilities|Text|ToText(String) (Utilities|String|Append (Utilities|String|Append (Utilities|String|Append (Utilities|String|ToString(Integer) (Class|KismetMathLibrary|GetHour _returnvalue)) (Variables|Default|GetSeperator)) (Utilities|String|ToString(Integer) (Class|KismetMathLibrary|GetMinute _returnvalue))) (Utilities|String|Append (Variables|Default|GetSeperator) (Utilities|String|ToString(Integer) (Class|KismetMathLibrary|GetSecond _returnvalue))))))
  (goto _label))

(fn ConstructionScript)