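; SwirlyBall is a test Blueprint for a ball that swirls in a circle until it is dropped.
; Tick advances a Speed-scaled timer and adds a cosine/sine local offset to the mesh without sweep, so movement per frame is not delta-scaled.
; DropSwirly stops the motion and turns on gravity and physics, while SetSpeed changes the swirl rate.
; The event binding for a group drop is never run.
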(event EventBeginPlay)

(event Collision|EventActorBeginOverlap
  (params (OtherActor :type Actor%20Object%20Reference)))

(event EventTick
  (params (DeltaSeconds :type Float%20%28single-precision%29))
  (bind _radius (Variables|Default|Getradius))
  ;[1 1 1] update timer with delta time
  (Variables|Default|Setcounter (+ (* DeltaSeconds (Variables|Default|Getspeed)) (Variables|Default|Getcounter)))
  (if (Variables|Default|GetisAlive)
    ;[1 1 1] move ball
    (Transformation|AddLocalOffset (Variables|Default|GetStaticMesh) (Math|Vector|MakeVector (* (Math|Trig|Cos(Radians) (Variables|Default|Getcounter)) _radius) (* (Math|Trig|Sin(Radians) (Variables|Default|Getcounter)) _radius) 0.0) false true)))

(fn ConstructionScript)

(fn DropSwirly
  (Physics|SetEnableGravity (Variables|Default|GetStaticMesh) true)
  (Variables|Default|SetisAlive false)
  (Physics|SetSimulatePhysics (Variables|Default|GetStaticMesh) true))

(fn SetSpeed
  (params (rad :type Float%20%28single-precision%29))
  (Variables|Default|Setspeed rad))