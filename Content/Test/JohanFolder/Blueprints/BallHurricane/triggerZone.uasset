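; Trigger zone actor for the BallHurricane test that lets the player drop every SwirlyBall by pressing J while the zone is occupied.
; It enables input from player controller 0 on BeginPlay, and unfiltered overlap events set the Inrange flag and toggle the glow on its referenced ballGround.
; A J press while Inrange is true calls DropSwirly on all SwirlyBall actors found in the level.
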(event EventBeginPlay
  ;[1 1 1] make it so that the zone can accept keyboard input
  (Input|EnableInput (Game|GetPlayerController 0)))

(event Collision|EventActorBeginOverlap
  (params (OtherActor :type Actor%20Object%20Reference))
  ;[1 1 1] entered zone
  (Variables|Default|Setinrange true)
  (Development|PrintString "Entered JZone")
  (bind _asball_ground (Utilities|Casting|CastToballGround (Variables|Default|Getground)))
  (Default|Glow _asball_ground))

(event EventTick
  (params (DeltaSeconds :type Float%20%28single-precision%29)))

(event Collision|EventActorEndOverlap
  (params (OtherActor :type Actor%20Object%20Reference))
  ;[1 1 1] left zone
  (Variables|Default|Setinrange false)
  (Development|PrintString "Left JZone")
  (bind _asball_ground (Utilities|Casting|CastToballGround (Variables|Default|Getground)))
  (Default|Unglow _asball_ground))

(event Input|KeyboardEvents|J
  (params (Key :type Key%20Structure :default "AnyKey"))
  ;[1 1 1] if pressing J & inside zone
  (:Pressed
    (if (Variables|Default|Getinrange)
      (Development|PrintString "Pressed J")
      ;;[1 1 1] tell all swirlyballs to drop
      (bind _outactors (Actor|GetAllActorsOfClass "/Game/Test/JohanFolder/Blueprints/BallHurricane/SwirlyBall.SwirlyBall_C"))
      (for _array_element _outactors
        (Default|DropSwirly _array_element)))))

(fn ConstructionScript)