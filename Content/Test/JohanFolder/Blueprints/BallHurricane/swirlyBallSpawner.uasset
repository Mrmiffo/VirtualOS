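; A test spawner actor that builds a vertical column of glowing SwirlyBall actors on BeginPlay.
; It spawns one hundred small balls stacked upward from its location, giving each a speed that grows with its height index and overriding the mesh with the Glowyswirly material.
; Leftover unconnected sine and cosine nodes suggest a ring offset that is currently not applied.
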(event EventBeginPlay
  (for _index (range 1 100)
    (bind _returnvalue (Game|SpawnActorfromClass "/Game/Test/JohanFolder/Blueprints/BallHurricane/SwirlyBall.SwirlyBall_C" (Math|Transform|MakeTransform (+ (Transformation|GetActorLocation) (Math|Vector|MakeVector 0.0 0.0 (Math|Conversions|ToFloat(Integer) (* _index 15)))) "0.000000,0.000000,0.000000" "0.200000,0.200000,0.200000") "AlwaysSpawn" 0 0))
    (Default|SetSpeed _returnvalue (* (Math|Conversions|ToFloat(Integer) _index) 0.1))
    (Rendering|Material|SetMaterial (Variables|/Game/Test/JohanFolder/Blueprints/BallHurricane/SwirlyBall.SwirlyBall_C|GetStaticMesh _returnvalue) 0 "/Game/Test/JohanFolder/Blueprints/BallHurricane/glowyswirly.glowyswirly")))

(fn ConstructionScript)