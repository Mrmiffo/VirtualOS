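; Analog clock actor whose second, minute and hour hands show the current system time.
; From BeginPlay, a looping one-second Delay reads Now and sets the relative pitch of each hand's scene component.
; Time values become negative angles with a 180-degree offset to keep the hands upright.
; The hour hand uses only the hour modulo twelve, so it jumps between hours rather than sweeping.
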(event EventBeginPlay
  (bind _returnvalue (Math|DateTime|Now))
  ;[1 1 1] Digital clock text, that updates every second.
  (Utilities|FlowControl|Delay 1.0 :!label _label)
  ;;[1 1 1] second
  (Transformation|SetRelativeRotation (Variables|Default|GetSecondHandScene) (Math|Rotator|MakeRotator 0.0 (+ (* (Math|Conversions|ToFloat(Integer) (Class|KismetMathLibrary|GetSecond _returnvalue)) -6.0) 1.8e+02) 0.0) false false)
  ;;[1 1 1] minute
  (Transformation|SetRelativeRotation (Variables|Default|Getminutehandscene) (Math|Rotator|MakeRotator 0.0 (+ (* (Class|KismetMathLibrary|GetMinute _returnvalue) -6.0) 1.8e+02) 0.0) false false)
  (Transformation|SetRelativeRotation (Variables|Default|GethourHandScene) (Math|Rotator|MakeRotator 0.0 (+ (* (Math|Integer|%(Integer) (Class|KismetMathLibrary|GetHour _returnvalue) 12) -3e+01) 1.8e+02) 0.0) false false)
  (goto _label))

(fn ConstructionScript)