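; Skybox Blueprint that switches the material on a sky sphere between two sky materials.
; The construction script applies the first material as the default.
; A custom Update event takes a Skybox value and applies the first material when it is below one, otherwise the second.
; BeginPlay, overlap and Tick are unused, so changes after construction depend on Update being called.
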(event EventBeginPlay)

(event Collision|EventActorBeginOverlap
  (params (OtherActor :type Actor%20Object%20Reference)))

(event EventTick
  (params (DeltaSeconds :type Float%20%28single-precision%29)))

(event EventUpdate
  (params (skybox :type Integer))
  (bind _skysphere (Variables|Default|GetSkySphere))
  (if (< skybox 1)
    (Rendering|Material|SetMaterial _skysphere 0 (Variables|Default|GetskyMaterial))
    (else
      (Rendering|Material|SetMaterial _skysphere 0 (Variables|Default|GetskyMaterial2)))))

(fn ConstructionScript
  (Rendering|Material|SetMaterial (Variables|Default|GetSkySphere) 0 (Variables|Default|GetskyMaterial)))