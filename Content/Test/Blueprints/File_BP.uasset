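; File_BP is an actor representing a file or folder as a 3D object that a motion controller can open and carry.
; Overlapping a motion controller while FileInteract is held calls OpenFile once.
; On FolderOpening it recursively spawns File_BP actors for the contained paths and attaches them in a centered, offset row.
; It also wraps long names on the label and attaches or detaches itself on Pickup and Drop.
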(event EventBeginPlay
  ;[1 1 1] Start listening to input from player on spawn
  (Input|EnableInput (Game|GetPlayerController 0)))

(event EventNameChanged
  (bind _name (Variables|Default|GetName))
  (bind _filenamerenderer (Variables|Default|GetFileNameRenderer))
  ;[1 1 1] Set the name in the name renderer
  (if (> (Utilities|String|Len _name) 9)
    (bind _stringwithbreak (CallFunction|AddBreakLinetoString 9 _name))
    (Rendering|Components|TextRender|SetText _filenamerenderer (Utilities|Text|ToText(String) _stringwithbreak))
    (else
      (Rendering|Components|TextRender|SetText _filenamerenderer (Utilities|Text|ToText(String) (Variables|Default|GetName))))))

(event Collision|EventActorBeginOverlap
  (params (OtherActor :type Actor%20Object%20Reference))
  ;[1 1 1] Open file on touch if interact is pressed
  (if (Math|Boolean|ANDBoolean (Utilities|ClassIsChildOf (Utilities|GetClass OtherActor) "/Game/Test/PlayerPawn/Blueprints/BP_MotionController.BP_MotionController_C") (Variables|Default|GetInteractOnTouch) (not (Variables|Default|GetFileIsOpen)))
    (Class|File|OpenFile)
    (Variables|Default|SetFileIsOpen true)))

(event EventPickup
  (params (AttachTo :type Scene%20Component%20Object%20Reference))
  (Transformation|AttachComponentToComponent (VehicleSound|GetRootComponent) AttachTo "None" "KeepWorld" "KeepWorld" "KeepWorld" true))

(event EventDrop
  (Transformation|DetachFromActor "KeepWorld" "KeepWorld" "KeepWorld"))

(event EventFolderOpening
  ;[1 1 1] Spawn and place new Files when opening folder
  (bind _spawnedfileobjects (CallFunction|SpawnFilesandFolders (Variables|Default|GetContentFiles) (Variables|Default|GetContentFolders)))
  (CallFunction|DisplayFilesandFolders _spawnedfileobjects))

(event Input|ActionEvents|InputActionFileInteract
  (params (Key :type Key%20Structure :default "AnyKey"))
  ;[1 1 1] FileInteractHandler
  (:Pressed
    (Variables|Default|SetInteractOnTouch true))
  (:Released
    (Variables|Default|SetInteractOnTouch false)))

(fn ConstructionScript
  (Rendering|Components|TextRender|SetText (Variables|Default|GetFileNameRenderer) (Utilities|Text|ToText(String) (Variables|Default|Getname))))

(fn SpawnFile
  (params (Path :type String) (Name :type String) (IsDirectory :type Boolean))
  (bind _returnvalue (Game|SpawnActorfromClass "File_BP_C" (Math|Transform|MakeTransform "0, 0, 0") "Undefined" 0 0))
  (Class|File|InitializeFile _returnvalue Path Name IsDirectory)
  (if IsDirectory
    _
    (else
      (Components|StaticMesh|SetStaticMesh (Variables|File_BP_C|GetFileModel _returnvalue) "/Game/TEMP_FILE.TEMP_FILE")))
  (return _returnvalue))

(fn SpawnFilesandFolders
  (params (Files :type Array%20of%20Strings) (Folders :type Array%20of%20Strings))
  (bind _filesandfolders (LocalVariables|GetFilesAndFolders))
  (for _array_element Files
    (bind _newfile (CallFunction|SpawnFile _array_element (Utilities|Array|Get(acopy) (Utilities|String|ParseIntoArray _array_element "/") (Utilities|Array|LastIndex (Utilities|String|ParseIntoArray _array_element "/"))) false))
    (Utilities|Array|Add _filesandfolders _newfile))
  (for _array_element_2 Folders
    (bind _newfile_2 (CallFunction|SpawnFile _array_element_2 (Utilities|Array|Get(acopy) (Utilities|String|ParseIntoArray _array_element_2 "/") (Utilities|Array|LastIndex (Utilities|String|ParseIntoArray _array_element_2 "/"))) true))
    (Utilities|Array|Add _filesandfolders _newfile_2))
  (return _filesandfolders))

(fn DisplayFilesandFolders
  (params (FileObjectsToDisplay :type Array%20of%20File%20BP%20Object%20References))
  (for (_array_element _array_index) FileObjectsToDisplay
    (Transformation|AttachActorToActor _array_element self "None" "SnapToTarget" "SnapToTarget" "SnapToTarget" true)
    (Transformation|AddLocalOffset (Variables|File_BP_C|GetDefaultSceneRoot _array_element) (Math|Vector|MakeVector 0.0 (+ (* _array_index (LocalVariables|GetDistanceBetweenFiles)) (* (- (Utilities|Array|Length FileObjectsToDisplay) 1) (/ (LocalVariables|GetDistanceBetweenFiles) -2.0))) (LocalVariables|GetDistanceToNextLineOfFiles)) false false)))

(fn AddBreakLinetoString
  (params (LineLength :type Integer) (String :type String))
  (bind _breaklinearray (LocalVariables|GetBreakLineArray))
  (for _index (range 0 (/ (Utilities|String|Len String) LineLength))
    ;[1 1 1] Add break by splitting into array and merging with seperating <br>
    (Utilities|Array|Add _breaklinearray (Utilities|String|GetSubstring String (* _index LineLength) LineLength)))
  (return (Utilities|String|JoinStringArray _breaklinearray "<br>")))