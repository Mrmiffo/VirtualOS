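; VRSimulatorPawn is a test pawn that rotates its camera from mouse axis input, apparently to simulate VR head look.
; MouseX and MouseY each subtract the current axis value from the stored previous value, then store the current one.
; The differences become single-axis vectors fed through MakeRotFromZ and MakeRotFromY into AddWorldRotation.
; These nodes treat the vectors as axis directions, so magnitude does not set the rotation angle.
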(event Input|MouseEvents|MouseX
  (params (AxisValue :type Float%20%28single-precision%29))
  (Utilities|FlowControl|Sequence
    (:then_0
      (Transformation|AddWorldRotation (Variables|Default|GetCamera) (Math|Rotator|MakeRotfromZ (Math|Vector|MakeVector 0.0 0.0 (- (Variables|Default|GetMouseLastFrameX) AxisValue))) false false))
    (:then_1
      (Variables|Default|SetMouseLastFrameX AxisValue))))

(event Input|MouseEvents|MouseY
  (params (AxisValue :type Float%20%28single-precision%29))
  (Utilities|FlowControl|Sequence
    (:then_0
      (Transformation|AddWorldRotation (Variables|Default|GetCamera) (Math|Rotator|MakeRotfromY (Math|Vector|MakeVector 0.0 (- (Variables|Default|GetMouseLastFrameY) AxisValue) 0.0)) false false))
    (:then_1
      (Variables|Default|SetMouseLastFrameY AxisValue))))

(fn ConstructionScript)