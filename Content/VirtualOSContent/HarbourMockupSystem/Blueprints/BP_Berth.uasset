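; BP_Berth is a berth actor in the harbour mockup, showing name, depth and length limits, and occupancy.
; Setup fills the text labels and calls SetTime, which formats the ETA, hides it at 00:00 and switches the mesh between green and red flag materials.
; DropObject uses the 00:00 text as its free check, then destroys the dropped ship icon and assigns a random ETA.
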(event Collision|EventActorBeginOverlap
  (params (OtherActor :type Actor%20Object%20Reference)))

(event EventTick
  (params (DeltaSeconds :type Float%20%28single-precision%29)))

(event EventDropObject
  (params (DropedObject :type Actor%20Object%20Reference))
  (if (Utilities|Enum|Equal(Enum) (Variables|/Script/Engine.TextRenderComponent|GetText (Variables|Default|GetETA)) (Utilities|Text|MakeLiteralText "00:00"))
    (bind _asbp_ship_icon (Utilities|Casting|CastToBP_ShipIcon DropedObject))
    (Actor|DestroyActor _asbp_ship_icon)
    (CallFunction|SetTime (Math|Random|RandomInteger 23) (Math|Random|RandomInteger 59))))

(fn ConstructionScript)

(fn Setup
  (params (Name :type String) (Depth :type Float%20%28single-precision%29) (Length :type Float%20%28single-precision%29) (Minutes :type Integer) (Hours :type Integer))
  (Rendering|Components|TextRender|SetText (Variables|Default|GetBerthName) (Utilities|Text|ToText(String) Name))
  (Rendering|Components|TextRender|SetText (Variables|Default|GetMaxDepth) (Utilities|Text|ToText(String) (Utilities|String|Append "D: " (Utilities|String|ToString(Float) Depth) " m")))
  (Rendering|Components|TextRender|SetText (Variables|Default|GetMaxLength) (Utilities|Text|ToText(String) (Utilities|String|Append "L: " (Utilities|String|ToString(Float) Length) " m")))
  (CallFunction|SetTime Hours Minutes))

(fn SetTime
  (params (Hour :type Integer) (Minute :type Integer))
  (bind _returnvalue (== Hour 0))
  (bind _returnvalue_2 (== Minute 0))
  (bind _eta (Variables|Default|GetETA))
  (bind _staticmesh (Variables|Default|GetStaticMesh))
  (bind _returnvalue_3 (and _returnvalue _returnvalue_2))
  (Rendering|Components|TextRender|SetText _eta (Utilities|Text|ToText(String) (Utilities|String|Append (Utilities|String|ToString(Text) (Utilities|Text|ToText(Integer) Hour true 2 2)) ":" (Utilities|String|ToString(Text) (Utilities|Text|ToText(Integer) Minute true 2 2)))))
  (Rendering|SetVisibility _eta (not _returnvalue_3) false)
  (if _returnvalue_3
    (Rendering|Material|SetMaterial _staticmesh 0 "/Game/VirtualOSContent/HarbourMockupSystem/Materials/M_FlagGreen.M_FlagGreen")
    (else
      (Rendering|Material|SetMaterial _staticmesh 0 "/Game/VirtualOSContent/HarbourMockupSystem/Materials/M_FlagRed.M_FlagRed"))))