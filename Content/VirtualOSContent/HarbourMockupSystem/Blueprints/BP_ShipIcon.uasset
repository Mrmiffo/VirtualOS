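; BP_ShipIcon is a grabbable ship marker for the harbour mockup, showing a ship's name, depth, length, requested harbour and national flag.
; Setup stores the ship data, writes it to text components and picks the flag mesh from the Flag value.
; StartGrab attaches it to the grabbing controller keeping world transform, and EndGrab detaches it only if that same controller releases it.
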(event EventBeginPlay)

(event Collision|EventActorBeginOverlap
  (params (OtherActor :type Actor%20Object%20Reference)))

(event EventEndGrab
  (params (ReleasingController :type Motion%20Controller%20Component%20Object%20Reference) (AltButtonPressed :type Boolean) (Thrown :type Boolean))
  (if (== ReleasingController (Variables|Default|GetGrabbingController))
    (Transformation|DetachFromActor "KeepWorld" "KeepWorld" "KeepWorld")))

(event EventTick
  (params (DeltaSeconds :type Float%20%28single-precision%29)))

(event EventStartGrab
  (params (GrabbingController :type Motion%20Controller%20Component%20Object%20Reference))
  (bind _output_get (Variables|Default|SetGrabbingController GrabbingController))
  (Transformation|AttachComponentToComponent _output_get "None" "KeepWorld" "KeepWorld" "KeepWorld" true))

(fn ConstructionScript)

(fn Setup
  (params (Depth :type Float%20%28single-precision%29) (Length :type Float%20%28single-precision%29) (Name :type String) (RequestedHarbour :type Harbour%20Enum) (Flag :type Country%20Enum))
  (bind _output_get (Variables|Default|SetDepthValue Depth))
  (bind _output_get_2 (Variables|Default|SetLengthValue Length))
  (bind _output_get_3 (Variables|Default|SetShipName Name))
  (Variables|Default|SetHarbourValue RequestedHarbour)
  (Rendering|Components|TextRender|SetText (Variables|Default|GetDepth) (Utilities|Text|ToText(String) (Utilities|String|Append "Depth: " (Utilities|String|ToString(Text) (Utilities|Text|ToText(Float) _output_get "HalfToEven" true 1 324 1 1)) " m")))
  (Rendering|Components|TextRender|SetText (Variables|Default|GetLength) (Utilities|Text|ToText(String) (Utilities|String|Append "Length: " (Utilities|String|ToString(Text) (Utilities|Text|ToText(Float) _output_get_2 "HalfToEven" true 1 324 1 1)) " m")))
  (Rendering|Components|TextRender|SetText (Variables|Default|GetName) (Utilities|Text|ToText(String) _output_get_3))
  (Rendering|Components|TextRender|SetText (Variables|Default|GetHarbour) (Utilities|Text|ToText(String) (Utilities|String|EnumtoString RequestedHarbour)))
  (switch Utilities|FlowControl|Switch|SwitchonCountry Flag
    (:NewEnumerator0
      (Components|StaticMesh|SetStaticMesh (Variables|Default|GetFlag) "/Game/VirtualOSContent/HarbourMockupSystem/Models/SwedishFlag.SwedishFlag"))
    (:NewEnumerator1
      (Components|StaticMesh|SetStaticMesh (Variables|Default|GetFlag) "/Game/VirtualOSContent/HarbourMockupSystem/Models/DanishFlag.DanishFlag"))
    (:NewEnumerator2
      (Components|StaticMesh|SetStaticMesh (Variables|Default|GetFlag) "/Game/VirtualOSContent/HarbourMockupSystem/Models/FinishFlag.FinishFlag"))
    (:NewEnumerator3
      (Components|StaticMesh|SetStaticMesh (Variables|Default|GetFlag) "/Game/VirtualOSContent/HarbourMockupSystem/Models/FrenchFlag.FrenchFlag"))
    (:NewEnumerator4
      (Components|StaticMesh|SetStaticMesh (Variables|Default|GetFlag) "/Game/VirtualOSContent/HarbourMockupSystem/Models/ItalyFlag.ItalyFlag"))
    (:NewEnumerator5
      (Components|StaticMesh|SetStaticMesh (Variables|Default|GetFlag) "/Game/VirtualOSContent/HarbourMockupSystem/Models/JapanFlag.JapanFlag"))))