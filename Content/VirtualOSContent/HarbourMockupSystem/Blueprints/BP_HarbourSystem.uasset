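; Harbour mockup actor that populates displays with a queue of incoming ships and the berths of the Arendal, Skandia, Skarvik, Alvsborg and Rya harbours.
; On BeginPlay, Fill functions pass hardcoded data to CreateShip and CreateBerth, which spawn BP_ShipIcon and BP_Berth actors and initialise them through Setup.
; Each actor snaps to its display start component and is spaced by a shared BerthNo counter, reset per list and for Skandia's second column.
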(event EventBeginPlay
  (CallFunction|FillIncoming)
  (CallFunction|FillArendal)
  (CallFunction|FillSkandia)
  (CallFunction|FillSkarvik)
  (CallFunction|FillAlvsborg)
  (CallFunction|FillRya))

(event Collision|EventActorBeginOverlap
  (params (OtherActor :type Actor%20Object%20Reference)))

(event EventTick
  (params (DeltaSeconds :type Float%20%28single-precision%29)))

(fn ConstructionScript)

(fn FillIncoming
  (Variables|Default|SetBerthNo 0)
  (CallFunction|CreateShip (Variables|Default|GetIncomingShipDisplayStart) "Bragfield" 8.0 1.7e+02 "NewEnumerator2" "NewEnumerator4")
  (CallFunction|CreateShip (Variables|Default|GetIncomingShipDisplayStart) "Danube" 10.3 2e+02 "NewEnumerator0" "NewEnumerator5")
  (CallFunction|CreateShip (Variables|Default|GetIncomingShipDisplayStart) "Abeille" 9.0 3e+02 "NewEnumerator0" "NewEnumerator3")
  (CallFunction|CreateShip (Variables|Default|GetIncomingShipDisplayStart) "Tonnant" 7.0 2.4e+02 "NewEnumerator1" "NewEnumerator1")
  (CallFunction|CreateShip (Variables|Default|GetIncomingShipDisplayStart) "Kilcurrig" 3.0 95.0 "NewEnumerator0" "NewEnumerator1")
  (CallFunction|CreateShip (Variables|Default|GetIncomingShipDisplayStart) "Börje" 3.0 58.0 "NewEnumerator1" "NewEnumerator0")
  (CallFunction|CreateShip (Variables|Default|GetIncomingShipDisplayStart) "Perkele" 3.0 95.0 "NewEnumerator0" "NewEnumerator2")
  (CallFunction|CreateShip (Variables|Default|GetIncomingShipDisplayStart) "Misu" 13.0 4e+02 "NewEnumerator1" "NewEnumerator5"))

(fn FillArendal
  (bind _arendaldisplaystart (Variables|Default|GetArendalDisplayStart))
  (Variables|Default|SetBerthNo 0)
  (CallFunction|CreateBerth "750" 9.3 2e+02 25 1 _arendaldisplaystart)
  (CallFunction|CreateBerth "750A" 9.0 0.0 0 0 _arendaldisplaystart)
  (CallFunction|CreateBerth "751" 9.0 3e+02 0 0 _arendaldisplaystart))

(fn FillSkandia
  (bind _skandiadisplaystart2 (Variables|Default|GetSkandiaDisplayStart2))
  (Variables|Default|SetBerthNo 0)
  (CallFunction|CreateBerth "600" 7.5 1.7e+02 10 2 (Variables|Default|GetSkandiaDisplayStart))
  (CallFunction|CreateBerth "601" 10.5 2.9e+02 0 0 (Variables|Default|GetSkandiaDisplayStart))
  (CallFunction|CreateBerth "610" 13.5 4e+02 5 0 (Variables|Default|GetSkandiaDisplayStart))
  (CallFunction|CreateBerth "613" 11.5 3.9e+02 0 0 (Variables|Default|GetSkandiaDisplayStart))
  (CallFunction|CreateBerth "615" 9.7 2e+02 30 10 (Variables|Default|GetSkandiaDisplayStart))
  (CallFunction|CreateBerth "640" 9.5 2.5e+02 59 0 (Variables|Default|GetSkandiaDisplayStart))
  (Variables|Default|SetBerthNo 0)
  (CallFunction|CreateBerth "641" 9.5 2.5e+02 0 0 _skandiadisplaystart2)
  (CallFunction|CreateBerth "642" 9.5 2.5e+02 48 0 _skandiadisplaystart2)
  (CallFunction|CreateBerth "643" 9.5 2.5e+02 0 0 _skandiadisplaystart2)
  (CallFunction|CreateBerth "644" 7.6 135.0 0 0 _skandiadisplaystart2))

(fn FillSkarvik
  (bind _skarvikdisplaystart (Variables|Default|GetSkarvikDisplayStart))
  (Variables|Default|SetBerthNo 0)
  (CallFunction|CreateBerth "506" 6.0 86.0 0 24 _skarvikdisplaystart)
  (CallFunction|CreateBerth "507" 6.5 85.0 0 0 _skarvikdisplaystart)
  (CallFunction|CreateBerth "508" 7.5 1.6e+02 0 0 _skarvikdisplaystart)
  (CallFunction|CreateBerth "509" 7.5 1.6e+02 0 0 _skarvikdisplaystart)
  (CallFunction|CreateBerth "510" 12.5 2.5e+02 2 0 _skarvikdisplaystart)
  (CallFunction|CreateBerth "511" 11.5 2e+02 0 0 _skarvikdisplaystart))

(fn FillAlvsborg
  (bind _alvsborgdisplaystart (Variables|Default|GetAlvsborgDisplayStart))
  (Variables|Default|SetBerthNo 0)
  (CallFunction|CreateBerth "700" 9.0 184.0 0 0 _alvsborgdisplaystart)
  (CallFunction|CreateBerth "702" 10.5 197.0 0 0 _alvsborgdisplaystart)
  (CallFunction|CreateBerth "710" 10.5 0.0 13 0 _alvsborgdisplaystart)
  (CallFunction|CreateBerth "711" 10.5 0.0 37 13 _alvsborgdisplaystart)
  (CallFunction|CreateBerth "712" 10.5 2.3e+02 1 0 _alvsborgdisplaystart)
  (CallFunction|CreateBerth "713" 8.5 2e+02 3 0 _alvsborgdisplaystart))

(fn FillRya
  (bind _ryadisplaystart (Variables|Default|GetRyaDisplayStart))
  (Variables|Default|SetBerthNo 0)
  (CallFunction|CreateBerth "551" 8.8 147.0 0 0 _ryadisplaystart)
  (CallFunction|CreateBerth "555" 7.3 1.6e+02 0 0 _ryadisplaystart)
  (CallFunction|CreateBerth "556 A" 7.3 1.1e+02 37 0 _ryadisplaystart)
  (CallFunction|CreateBerth "556 B" 7.3 1.1e+02 0 0 _ryadisplaystart)
  (CallFunction|CreateBerth "556 C" 3.8 67.0 0 0 _ryadisplaystart))

(fn CreateBerth
  (params (Name :type String) (Depth :type Float%20%28single-precision%29) (Length :type Float%20%28single-precision%29) (Minutes :type Integer) (Hours :type Integer) (Start :type Scene%20Component%20Object%20Reference))
  (bind _returnvalue (Game|SpawnActorfromClass "/Game/VirtualOSContent/HarbourMockupSystem/Blueprints/BP_Berth.BP_Berth_C" (Math|Transform|MakeTransform "0, 0, 0" "0, 0, 0" "0.800000,0.800000,0.800000") "Undefined" 0 0))
  (Transformation|AttachComponentToComponent _returnvalue Start "None" "SnapToTarget" "SnapToTarget" "KeepWorld" true)
  (Transformation|AddActorLocalOffset _returnvalue (* (Variables|Default|GetOffset) (Variables|Default|GetBerthNo)) false false)
  (Math|Integer|IncrementInt (Variables|Default|GetBerthNo)
    (:%20%20
      (Default|Setup _returnvalue Name Depth Length Minutes Hours))))

(fn CreateShip
  (params (Origin :type Scene%20Component%20Object%20Reference) (Name :type String) (Depth :type Float%20%28single-precision%29) (Length :type Float%20%28single-precision%29) (Harbour :type Harbour%20Enum) (Flag :type Country%20Enum))
  (bind _returnvalue (Game|SpawnActorfromClass "/Game/VirtualOSContent/HarbourMockupSystem/Blueprints/BP_ShipIcon.BP_ShipIcon_C" (Math|Transform|MakeTransform "0, 0, 0" "0, 0, 0" "0.600000,0.600000,0.600000") "Undefined" 0 0))
  (Transformation|AttachComponentToComponent _returnvalue Origin "None" "SnapToTarget" "SnapToTarget" "KeepWorld" true)
  (Transformation|AddActorLocalOffset _returnvalue (* (LocalVariables|GetShipOffset) (Variables|Default|GetBerthNo)) false false)
  (Default|Setup _returnvalue Depth Length Name Harbour Flag)
  (Math|Integer|IncrementInt (Variables|Default|GetBerthNo)))