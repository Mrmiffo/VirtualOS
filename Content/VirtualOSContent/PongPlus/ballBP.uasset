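; Ball actor for the PongPlus game that reports overlaps and can be shattered.
; Its box forwards each overlapped actor to the Pong reference supplied through SetPong, leaving collision response to that object.
; GetColliding returns any overlapping PaddleAI actors.
; Destroy applies heavy damage to the BallDM destructible component with an impulse along a given X/Y direction.
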(event OnComponentBeginOverlap(Box)
  (params (OverlappedComponent :type Primitive%20Component%20Object%20Reference) (OtherActor :type Actor%20Object%20Reference) (OtherComp :type Primitive%20Component%20Object%20Reference) (OtherBodyIndex :type Integer) (bFromSweep :type Boolean) (SweepResult :type Hit%20Result%20Structure%20%28by%20ref%29))
  (bind _pong (Variables|Default|Getpong))
  (if (Utilities|IsValid _pong)
    (Default|BallCollided _pong OtherActor)))

(event EventBeginPlay)

(event Collision|EventActorBeginOverlap
  (params (OtherActor :type Actor%20Object%20Reference)))

(event EventTick
  (params (DeltaSeconds :type Float%20%28single-precision%29)))

(fn ConstructionScript)

(fn GetColliding
  (bind _box (Variables|Default|GetBox))
  (bind _overlappingactors (Collision|GetOverlappingActors _box "/Game/VirtualOSContent/PongPlus/PaddleAI.PaddleAI_C" :!class /Script/Engine.PrimitiveComponent))
  (if (> (Utilities|Array|Length _overlappingactors) 0)
    (return _overlappingactors)))

(fn Destroy
  (params (x :type Float%20%28single-precision%29) (y :type Float%20%28single-precision%29))
  (Game|Damage|ApplyDamage (Variables|Default|Getball_DM) 1e+03 (Transformation|GetWorldLocation (Variables|Default|Getball_DM)) (Math|Vector|MakeVector x y 0.0) 5.0))

(fn SetPong
  (params (pong :type Pong%20Object%20Reference))
  (Variables|Default|Setpong pong))