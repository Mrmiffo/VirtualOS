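; A grabbable VirtualOS panel that holds a grid of ProgramSnappoints on a backplate, 2x4 on startup.
; Setup spawns an attached Snapgrid, adds or removes non-grabbable snappoints to match the requested size, snaps them to the grid and scales the backplate.
; Grabbing attaches the panel to the controller; a thrown release enables backplate physics, then destroys the panel and its spawned actors after a delay.
; The program hologram, name and running-state functions are empty stubs.
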(event EventStartGrab
  (params (GrabbingController :type Motion%20Controller%20Component%20Object%20Reference))
  ;[1 1 1] Grab
  ;;[1 1 1] Attach to hand
  (bind _output_get (Variables|Default|SetGrabbingController GrabbingController))
  (Transformation|AttachComponentToComponent (Variables|Default|GetDefaultSceneRoot) _output_get "None" "KeepWorld" "KeepWorld" "KeepWorld" true))

(event EventOnStartup
  (params (startParams :type String))
  ;[1 1 1] Setup a default grid of 3x3 on startup
  (CallFunction|Setup 2 4 3e+01 4e+01))

(event EventEndGrab
  (params (ReleasingController :type Motion%20Controller%20Component%20Object%20Reference) (AltButtonPressed :type Boolean) (Thrown :type Boolean))
  ;[1 1 1] Grab
  ;;[1 1 1] Detach from hand if t was the grabbing hand
  (if (== ReleasingController (Variables|Default|GetGrabbingController))
    (Transformation|DetachFromActor "KeepWorld" "KeepWorld" "KeepWorld")
    ;;[1 1 1] Destroy actor if it was thrown
    (if Thrown
      (Physics|SetSimulatePhysics (Variables|Default|GetBackplate) true)
      (Utilities|FlowControl|Delay 2.0)
      (CallFunction|Kill))))

(event EventKill
  ;[1 1 1] Cleanup spawned stuff
  (for _array_element (Variables|Default|GetSnappoints)
    (Default|Kill _array_element))
  (Default|Kill (Variables|Default|GetSnapgrid))
  (Actor|DestroyActor))

(fn ConstructionScript)

(fn Setup
  (params (Rows :type Integer) (Columns :type Integer) (SpreadWidth :type Float%20%28single-precision%29) (SpreadHeight :type Float%20%28single-precision%29))
  (bind _returnvalue (* Columns SpreadWidth))
  (bind _returnvalue_2 (* Rows SpreadHeight))
  (bind _returnvalue_3 (* Rows Columns))
  (Utilities|IsValid (Variables|Default|GetSnapgrid)
    (:Is%20Valid
      _)
    (:Is%20Not%20Valid
      (bind _returnvalue_4 (Game|SpawnActorfromClass "/Game/VirtualOSContent/Snapgrid/Snapgrid.Snapgrid_C" (Transformation|GetWorldTransform (Variables|Default|GetDefaultSceneRoot)) "Undefined" 0 0))
      (bind _output_get (Variables|Default|SetSnapgrid _returnvalue_4))
      (Transformation|AttachComponentToComponent _output_get (Variables|Default|GetDefaultSceneRoot) "None" "SnapToTarget" "SnapToTarget" "SnapToTarget" true)))
  (Default|Setup (Variables|Default|GetSnapgrid) Columns Rows _returnvalue _returnvalue_2 "NewEnumerator0")
  (for _index (range (+ (Utilities|Array|Length (Variables|Default|GetSnappoints)) 1) _returnvalue_3)
    ;[1 1 1] Fill up with snappoints
    (bind _returnvalue_5 (Game|SpawnActorfromClass "/Game/VirtualOSContent/ProgramSnappoint/Blueprints/ProgramSnappoint.ProgramSnappoint_C" (Transformation|GetWorldTransform (Variables|Default|GetDefaultSceneRoot)) "Undefined" 0 0))
    (Utilities|Array|Add (Variables|Default|GetSnappoints) _returnvalue_5)
    (Variables|/Game/VirtualOSContent/ProgramSnappoint/Blueprints/ProgramSnappoint.ProgramSnappoint_C|SetGrabable _returnvalue_5 false))
  ;[1 1 1] Remove excess snappoints if the size was reduced
  (bind (_arrayindex _arrayelement) (Utilities|Array|ReverseforEachLoop (Variables|Default|GetSnappoints))
    (:LoopBody
      (if (>= _arrayindex _returnvalue_3)
        (Utilities|Array|RemoveItem (Variables|Default|GetSnappoints) _arrayelement)
        (Utilities|IsValid _arrayelement
          (:Is%20Valid
            (Default|Kill _arrayelement)))))
    (:Completed
      ;[1 1 1] Snap the snappoints to the grid
      (Default|AttachList (Variables|Default|GetSnapgrid) (Variables|Default|GetSnappoints))
      (Transformation|SetWorldScale3D (Variables|Default|GetBackplate) (Math|Vector|MakeVector 1.0 (/ _returnvalue 1.2e+02) (/ _returnvalue_2 8e+01))))))

(fn GetProgramHologram
  (return 0))

(fn GetProgramName
  (return ""))

(fn IsRunning
  (return false))