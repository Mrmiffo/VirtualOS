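; Shelf actor in the virtual OS content that provides a grid of ProgramSnappoint slots, presumably for placing programs.
; On BeginPlay it spawns a three-by-three grid of snappoints, attaches each to itself and offsets it locally using ItemSpacing across Y and ShelfHeight up Z.
; Each snappoint is stored in the Snappoints array and has EndIndication called so it starts without its indication.
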(event EventBeginPlay
  (for _index (range 0 2)
    (for _index_2 (range 0 2)
      (bind _returnvalue (Game|SpawnActorfromClass "/Game/VirtualOSContent/ProgramSnappoint/Blueprints/ProgramSnappoint.ProgramSnappoint_C" (Math|Transform|MakeTransform "0, 0, 0") "Undefined" 0 0))
      (Transformation|AttachActorToActor _returnvalue self "None" "SnapToTarget" "SnapToTarget" "SnapToTarget" true)
      (Transformation|AddActorLocalOffset _returnvalue (Math|Vector|MakeVector 0.0 (- (* _index_2 (Variables|Default|GetItem%20spacing)) 35.0) (+ (* _index (Variables|Default|GetShelf%20height)) 7.0)) false true)
      (Utilities|Array|Add (Variables|Default|GetSnappoints) _returnvalue)
      (Default|EndIndication _returnvalue))))

(fn ConstructionScript)