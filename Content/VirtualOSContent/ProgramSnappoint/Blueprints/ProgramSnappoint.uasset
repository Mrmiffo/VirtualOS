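; ProgramSnappoint is a snap target actor that pulls dropped objects to its position and rotation, then attaches them.
; LerpHelper components drive both the snap and a pulsing indicator sphere, chaining through completion callbacks.
; Start and EndIndication toggle the pulse, sphere visibility and collision.
; When Grabable, it follows the grabbing controller, then on release snaps its rotation to degree steps or, if thrown, simulates sphere physics before destroying itself.
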(event EventDropObject
  (params (DropedObject :type Actor%20Object%20Reference))
  (bind _defaultsceneroot (Variables|Default|GetDefaultSceneRoot))
  (bind _returnvalue (Transformation|GetWorldTransform _defaultsceneroot))
  (bind (_location _rotation) (Math|Transform|BreakTransform _returnvalue))
  ;[1 1 1] Lerp the droped object to the snappoint
  ;;[1 1 1] Lerp helper only work in local space
  (bind _returnvalue_2 (AddComponent|AddLerpHelper false))
  (Default|LerpTransformActorWorld _returnvalue_2 0.2 (Math|Transform|MakeTransform _location _rotation (Transformation|GetActorScale3D DropedObject)) DropedObject self))

(event EventLerpDoneActor
  (params (LerpHelper :type Lerp%20Helper%20Object%20Reference) (LerpedActor :type Actor%20Object%20Reference))
  ;[1 1 1] Attach the actor to the snappoint and destroy the lerper
  (Components|DestroyComponent LerpHelper)
  (Transformation|AttachActorToActor LerpedActor self "None" "KeepWorld" "KeepWorld" "KeepWorld" true))

(event EventBeginPlay
  (CallFunction|StartIndication))

(event EventEndGrab
  (params (ReleasingController :type Motion%20Controller%20Component%20Object%20Reference) (AltButtonPressed :type Boolean) (Thrown :type Boolean))
  (bind _returnvalue (Transformation|GetActorRotation))
  (bind _snaptorotationdegree (Variables|Default|GetSnapToRotationDegree))
  (bind (_roll _pitch _yaw) (Math|Rotator|BreakRotator _returnvalue))
  ;[1 1 1] Simply move with hand on grab
  (if (== ReleasingController (Variables|Default|GetGrabbingController))
    (Transformation|DetachFromActor "KeepWorld" "KeepWorld" "KeepWorld")
    ;[1 1 1] Throw away and destroy if thrown
    (if Thrown
      (Physics|SetSimulatePhysics (Variables|Default|GetIndicatorSphere) true)
      (Utilities|FlowControl|Delay 2.0)
      (CallFunction|Kill)
      (else
        (Transformation|SetActorRotation (Math|Rotator|MakeRotator (* (Math|Float|Round (/ _roll _snaptorotationdegree)) _snaptorotationdegree) (* (Math|Float|Round (/ _pitch _snaptorotationdegree)) _snaptorotationdegree) (* (Math|Float|Round (/ _yaw _snaptorotationdegree)) _snaptorotationdegree)))))))

(event EventStartGrab
  (params (GrabbingController :type Motion%20Controller%20Component%20Object%20Reference))
  ;[1 1 1] Simply move with hand on grab
  (if (Variables|Default|GetGrabable)
    (bind _output_get (Variables|Default|SetGrabbingController GrabbingController))
    (Transformation|AttachComponentToComponent _output_get "None" "KeepWorld" "KeepWorld" "KeepWorld" true)))

(event EventKill
  (bind _animationlerphelper (Variables|Default|GetAnimationLerpHelper))
  ;[1 1 1] Destroy the animation componenet if it exists
  (Utilities|IsValid _animationlerphelper
    (:Is%20Valid
      (Components|DestroyComponent _animationlerphelper))
    (:Is%20Not%20Valid
      _))
  (Actor|DestroyActor))

(event EventLerpDoneComponent
  (params (LerpHelper :type Lerp%20Helper%20Object%20Reference) (Component :type Scene%20Component%20Object%20Reference))
  (bind _returnvalue (Transformation|GetRelativeTransform Component))
  (bind (_location _rotation) (Math|Transform|BreakTransform _returnvalue))
  ;[1 1 1] Indication animation
  (if (Variables|Default|GetIndicationRunning)
    (if (Variables|Default|GetShrinking)
      (Variables|Default|SetNextTransform (Math|Transform|MakeTransform _location _rotation "1.000000,1.000000,1.000000"))
      (else
        (Variables|Default|SetNextTransform (Math|Transform|MakeTransform _location _rotation "0.500000,0.500000,0.500000"))))
    (Variables|Default|SetShrinking (not (Variables|Default|GetShrinking)))
    (Default|LerpTransformComponent LerpHelper 1.0 (Variables|Default|GetNextTransform) self (Variables|Default|GetIndicatorSphere))))

(fn ConstructionScript)

(fn StartIndication
  (bind _indicatorsphere (Variables|Default|GetIndicatorSphere))
  (bind _returnvalue (Transformation|GetRelativeTransform _indicatorsphere))
  (bind (_location _rotation) (Math|Transform|BreakTransform _returnvalue))
  (Variables|Default|SetShrinking false)
  (Variables|Default|SetIndicationRunning true)
  (Collision|SetActorEnableCollision true)
  (Transformation|SetRelativeScale3D _indicatorsphere "0.100000,0.100000,0.100000")
  (Rendering|SetVisibility _indicatorsphere true true)
  (bind _returnvalue_2 (AddComponent|AddLerpHelper false))
  (bind _output_get (Variables|Default|SetAnimationLerpHelper _returnvalue_2))
  (Default|LerpTransformComponent _output_get 1.0 (Math|Transform|MakeTransform _location _rotation "1.000000,1.000000,1.000000") self (Variables|Default|GetIndicatorSphere)))

(fn EndIndication
  (bind _animationlerphelper (Variables|Default|GetAnimationLerpHelper))
  (Rendering|SetVisibility (Variables|Default|GetIndicatorSphere) false true)
  (Variables|Default|SetIndicationRunning false)
  (Collision|SetActorEnableCollision false)
  (Utilities|IsValid _animationlerphelper
    (:Is%20Valid
      (Components|DestroyComponent _animationlerphelper))))