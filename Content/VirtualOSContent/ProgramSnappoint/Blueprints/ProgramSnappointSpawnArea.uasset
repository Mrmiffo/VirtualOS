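; Grabbable spawn area that creates new ProgramSnappoint actors in the virtual OS.
; On grab, it spawns a snappoint at its root location and forwards the grab to it, then passes the release on to that same snappoint.
; Its indicator mesh pulses continuously between two scales, with each LerpHelper completion callback toggling a flag and starting the next lerp.
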(event EventBeginPlay
  ;[1 1 1] Start morphing when spawned
  (CallFunction|LerpDoneComponent (Variables|Default|GetLerpHelper) (Variables|Default|GetIndicatorMesh)))

(event EventStartGrab
  (params (GrabbingController :type Motion%20Controller%20Component%20Object%20Reference))
  ;[1 1 1] Create a new snappoint when grabed
  (bind _returnvalue (Game|SpawnActorfromClass "/Game/VirtualOSContent/ProgramSnappoint/Blueprints/ProgramSnappoint.ProgramSnappoint_C" (Math|Transform|MakeTransform (.Location (Math|Transform|BreakTransform (Transformation|GetWorldTransform (Variables|Default|GetDefaultSceneRoot))))) "Undefined" 0 0))
  (Default|StartGrab _returnvalue GrabbingController))

(event EventEndGrab
  (params (ReleasingController :type Motion%20Controller%20Component%20Object%20Reference) (AltButtonPressed :type Boolean) (Thrown :type Boolean))
  ;[1 1 1] Release the spawned snappoint when hand release
  (Default|EndGrab (stale EventStartGrab _returnvalue) ReleasingController AltButtonPressed Thrown))

(event EventLerpDoneComponent
  (params (LerpHelper :type Lerp%20Helper%20Object%20Reference) (Component :type Scene%20Component%20Object%20Reference))
  (bind _returnvalue (Transformation|GetRelativeTransform (Variables|Default|GetLerpHelper)))
  (bind (_location _rotation) (Math|Transform|BreakTransform _returnvalue))
  (if (Variables|Default|GetShrinking)
    (Variables|Default|SetNewScale "0.100000,0.100000,0.100000")
    (else
      (Variables|Default|SetNewScale "0.050000,0.050000,0.050000")))
  (Variables|Default|SetShrinking (not (Variables|Default|GetShrinking)))
  (Default|LerpTransformComponent LerpHelper 1.0 (Math|Transform|MakeTransform _location _rotation (Variables|Default|GetNewScale)) self Component))

(event EventKill
  (Actor|DestroyActor))

(fn ConstructionScript)