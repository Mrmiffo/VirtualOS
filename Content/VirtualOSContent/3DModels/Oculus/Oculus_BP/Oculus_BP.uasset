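; Grabbable Oculus object Blueprint that can be held by a controller and can launch the VRGame level through its Start event.
; StartGrab records the controller and attaches the root to it, keeping world transform.
; EndGrab responds only to that controller: a throw enables physics on the Oculus component and destroys the actor after a short delay, while a normal release just detaches it.
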(event EventBeginPlay)

(event Collision|EventActorBeginOverlap
  (params (OtherActor :type Actor%20Object%20Reference)))

(event EventStartGrab
  (params (GrabbingController :type Motion%20Controller%20Component%20Object%20Reference))
  ;[1 1 1] Grab and release
  (bind _output_get (Variables|Default|SetGrabbingController GrabbingController))
  (Transformation|AttachComponentToComponent (Variables|Default|GetDefaultSceneRoot) _output_get "None" "KeepWorld" "KeepWorld" "KeepWorld" true))

(event EventTick
  (params (DeltaSeconds :type Float%20%28single-precision%29)))

(event EventEndGrab
  (params (ReleasingController :type Motion%20Controller%20Component%20Object%20Reference) (AltButtonPressed :type Boolean) (Thrown :type Boolean))
  ;[1 1 1] Grab and release
  (if (== ReleasingController (Variables|Default|GetGrabbingController))
    (if Thrown
      (Physics|SetSimulatePhysics (Variables|Default|GetOculus) true)
      (Utilities|FlowControl|Delay 2.0)
      (Actor|DestroyActor)
      (else
        (Transformation|DetachFromActor "KeepWorld" "KeepWorld" "KeepWorld")))))

(event EventStart
  (params (Args :type String))
  (Game|OpenLevel(byName) "VRGame"))

(fn ConstructionScript)