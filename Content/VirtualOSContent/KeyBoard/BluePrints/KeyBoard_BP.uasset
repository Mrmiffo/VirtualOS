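; KeyBoard_BP is a grabbable virtual keyboard actor that acts as a VirtualOS program, reporting its name, hologram and an always-running state.
; On BeginPlay it hands its WidgetInteraction component to the KeyBoard_WB widget for keyboard input.
; Grabbing attaches it to the controller; releasing detaches it, while throwing enables physics on the cube and destroys the actor after a short delay.
; Leftover answer-checking logic is unconnected.
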(event Custom|SendPressed_Event_0
  ;[1 1 1] Junk that can be deleted when done...
)

(event EventBeginPlay
  ;[1 1 1] Getting keyboard inputs.
  (bind _askey_board_wb (Utilities|Casting|CastToKeyBoard_WB (UserInterface|GetUserWidgetObject (Variables|Default|GetWidget))))
  (Variables|/Game/VirtualOSContent/KeyBoard/Widgets/KeyBoard_WB.KeyBoard_WB_C|SetWidgetInteraction _askey_board_wb (Variables|Default|GetWidgetInteraction)))

(event Collision|EventActorBeginOverlap
  (params (OtherActor :type Actor%20Object%20Reference)))

(event EventStartGrab
  (params (GrabbingController :type Motion%20Controller%20Component%20Object%20Reference))
  ;[1 1 1] Grab and release
  (bind _output_get (Variables|Default|SetGrabbingController GrabbingController))
  (Transformation|AttachComponentToComponent (Variables|Default|GetDefaultSceneRoot) _output_get "None" "KeepWorld" "KeepWorld" "KeepWorld" true))

(event EventTick
  (params (DeltaSeconds :type Float%20%28single-precision%29)))

(event EventEndGrab
  (params (ReleasingController :type Motion%20Controller%20Component%20Object%20Reference) (AltButtonPressed :type Boolean) (Thrown :type Boolean))
  ;[1 1 1] Grab and release
  (if (== ReleasingController (Variables|Default|GetGrabbingController))
    (if Thrown
      (Physics|SetSimulatePhysics (Variables|Default|GetCube) true)
      (Utilities|FlowControl|Delay 2.0)
      (Actor|DestroyActor)
      (else
        (Transformation|DetachFromActor "KeepWorld" "KeepWorld" "KeepWorld")))))

(fn ConstructionScript)

(fn GetProgramHologram
  (return "/Game/Geometry/Meshes/1M_Cube.1M_Cube"))

(fn GetProgramName
  (return (Variables|Default|GetName)))

(fn IsRunning
  (return true))