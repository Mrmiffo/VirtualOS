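; Skybox actor that mirrors live weather from a web JSON request, re-fetched about every 30 minutes through a delayed Tick.
; The response's wind speed becomes one of four tiers, and its condition text is matched against lightning, rain, cloud, partly-cloud and sun groups.
; ChangeWeather then drives cloud opacity, color and speed on a dynamic sky material and toggles rain.
; Flag-checked delay loops replay rain, sun and strong-wind audio.
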(event Custom|CustomEvent
  (params (bSuccess :type Boolean) (JSON :type Json%20Field%20Data%20Object%20Reference) (Status :type EJSONResult%20Enum))
  (bind (_success _returnvalue) (Class|JsonFieldData|GetObject JSON "query"))
  (bind _returnvalue_2 (Class|JsonFieldData|GetObject _returnvalue "results"))
  (bind _returnvalue_3 (Class|JsonFieldData|GetObject _returnvalue_2 "channel"))
  (bind _returnvalue_4 (Class|JsonFieldData|GetObject _returnvalue_3 "wind"))
  (bind _returnvalue_5 (Class|JsonFieldData|GetObject _returnvalue_3 "item"))
  (bind _returnvalue_6 (Class|JsonFieldData|GetString _returnvalue_4 "speed"))
  (bind _returnvalue_7 (Class|JsonFieldData|GetObject _returnvalue_5 "condition"))
  (bind (_success_2 _returnvalue_8) (Class|JsonFieldData|GetString _returnvalue_7 "text"))
  (bind _returnvalue_9 (Math|Conversions|ToFloat(Integer) _returnvalue_6))
  (bind _returnvalue_10 (* _returnvalue_9 0.44704))
  (bind _returnvalue_11 (Math|Float|Round _returnvalue_10))
  (if bSuccess
    (if _success
      (Variables|Default|SetIsRaining false)
      (Variables|Default|SetIsSunny false)
      (Variables|Default|SetIsReallyWindy false)
      (CallFunction|StopAllAudio)
      (Utilities|FlowControl|Sequence
        (:then_0
          (if (< _returnvalue_11 6)
            (Variables|Default|SetWindSpeed 1)
            (elif (< _returnvalue_11 11)
              (Variables|Default|SetWindSpeed 2)
              (elif (< _returnvalue_11 16)
                (Variables|Default|SetWindSpeed 3)
                (else
                  (Variables|Default|SetWindSpeed 4)
                  (Variables|Default|SetIsReallyWindy true)
                  (CallFunction|PlayAudio "Windy" :!label _label)
                  (if (Variables|Default|GetIsReallyWindy)
                    (Utilities|FlowControl|Delay 1.8e+02)
                    (goto _label)))))))
        (:then_1
          (if _success_2
            (for _array_element (Variables|Default|GetGroupLightning)
              (if (Utilities|Enum|Equal(Enum) _array_element _returnvalue_8)
                (CallFunction|ChangeWeather "Raining" (Variables|Default|GetWindSpeed))
                (Variables|Default|SetIsRaining true)
                (CallFunction|PlayAudio "Rain" :!label _label_2)
                (if (Variables|Default|GetIsRaining)
                  (Utilities|FlowControl|Delay 28.0)
                  (goto _label_2))))
            (for _array_element_2 (Variables|Default|GetGroupRain)
              (if (Utilities|Enum|Equal(Enum) _array_element_2 _returnvalue_8)
                (CallFunction|ChangeWeather "Raining" (Variables|Default|GetWindSpeed))
                (Variables|Default|SetIsRaining true)
                (CallFunction|PlayAudio "Rain" :!label _label_3)
                (if (Variables|Default|GetIsRaining)
                  (Utilities|FlowControl|Delay 28.0)
                  (goto _label_3))))
            (for _array_element_3 (Variables|Default|GetGroupCloud)
              (if (Utilities|Enum|Equal(Enum) _array_element_3 _returnvalue_8)
                (CallFunction|ChangeWeather "Cloudy" (Variables|Default|GetWindSpeed))))
            (for _array_element_4 (Variables|Default|GetGroupPartlyCloud)
              (if (Utilities|Enum|Equal(Enum) _array_element_4 _returnvalue_8)
                (CallFunction|ChangeWeather "PartlyCloud" (Variables|Default|GetWindSpeed))))
            (for _array_element_5 (Variables|Default|GetGroupSun)
              (if (Utilities|Enum|Equal(Enum) _array_element_5 _returnvalue_8)
                (CallFunction|ChangeWeather "Sun/Clear" (Variables|Default|GetWindSpeed))
                (Variables|Default|SetIsSunny true)
                (CallFunction|PlayAudio "Sun" :!label _label_4)
                (if (Variables|Default|GetIsSunny)
                  (Utilities|FlowControl|Delay 2e+01)
                  (goto _label_4))))
            (else
              (Development|PrintString "Could not get current weather. Retrying in 10 sec...")
              (Utilities|FlowControl|Delay 1e+01)
              (CallFunction|TrytoGetWeather)))))
      (else
        (Development|PrintString "Could not get object field")))
    (else
      (Development|PrintString "OnGetResult Failed"))))

(event Custom|Try%20to%20get%20weather
  (bind _returnvalue (Class|JsonFieldData|GetRequest (Class|JsonFieldData|Create) (Variables|Default|GetURL)))
  (if (Utilities|IsValid _returnvalue)
    (EventDispatchers|AssignOnGetResult _returnvalue (delegate Custom|CustomEvent))
    (else
      (Development|PrintString "JSON Request Failed"))))

(event EventBeginPlay
  (CallFunction|InitiateVariables))

(event EventTick
  (params (DeltaSeconds :type Float%20%28single-precision%29))
  (if (Variables|Default|GetFirstTime)
    (Variables|Default|SetFirstTime false)
    (else
      (Utilities|FlowControl|Delay 1.8e+03)))
  (bind _returnvalue (Class|JsonFieldData|GetRequest (Class|JsonFieldData|Create) (Variables|Default|GetURL)))
  (if (Utilities|IsValid _returnvalue)
    (EventDispatchers|AssignOnGetResult _returnvalue (delegate Custom|CustomEvent))
    (else
      (Development|PrintString "JSON Request Failed"))))

(fn ConstructionScript)

(fn InitiateVariables
  (bind _returnvalue (Rendering|Material|CreateDynamicMaterialInstance (Variables|Default|GetSkySphere) 0 "/Engine/EngineSky/M_Sky_Panning_Clouds2.M_Sky_Panning_Clouds2" :!class /Script/Engine.PrimitiveComponent))
  (Variables|Components|SetMaterial%20Instance _returnvalue))

(fn ChangeWeather
  (params (Weather :type String) (WindSpeed :type Integer))
  (bind _material_instance (Variables|Components|GetMaterial%20Instance))
  (bind _material_instance_2 (Variables|Components|GetMaterial%20Instance))
  (bind _material_instance_3 (Variables|Components|GetMaterial%20Instance))
  (bind _material_instance_4 (Variables|Components|GetMaterial%20Instance))
  (Variables|Default|SetWindSpeed WindSpeed)
  (Variables|Default|SetInput Weather)
  (Components|Activation|SetActive (Variables|Default|GetRain) false false)
  (Utilities|FlowControl|Sequence
    (:then_0
      (if (== (Variables|Default|GetWindSpeed) 1)
        (Variables|Default|SetCloudSpeed 5.0)
        (elif (== (Variables|Default|GetWindSpeed) 2)
          (Variables|Default|SetCloudSpeed 1e+01)
          (elif (== (Variables|Default|GetWindSpeed) 3)
            (Variables|Default|SetWindSpeed 20)
            (else
              (Variables|Default|SetWindSpeed 40))))))
    (:then_1
      (if (Utilities|Enum|Equal(Enum) (Variables|Default|GetInput) (Variables|Default|GetSun))
        (Variables|Default|SetCloudOpacity 0.2)
        (Variables|Components|SetCloud%20color "(R=1.000000,G=1.000000,B=1.000000,A=1.000000)")
        ;[1 1 1] Sun/Clear
        (Rendering|Material|SetScalarParameterValue _material_instance_3 "Cloud opacity" (Variables|Default|GetCloudOpacity) :!class /Script/Engine.MaterialInstanceDynamic)
        (Rendering|Material|SetVectorParameterValue _material_instance_3 "Cloud color" (Variables|Components|GetCloud%20color) :!class /Script/Engine.MaterialInstanceDynamic)
        (Rendering|Material|SetScalarParameterValue _material_instance_3 "Cloud speed" (Variables|Default|GetCloudSpeed) :!class /Script/Engine.MaterialInstanceDynamic)
        (return)
        (elif (Utilities|Enum|Equal(Enum) (Variables|Default|GetInput) (Variables|Default|GetRaining))
          (Variables|Default|SetCloudOpacity 7.0)
          (Variables|Components|SetCloud%20color "(R=0.120000,G=0.120000,B=0.120000,A=1.000000)")
          ;[1 1 1] Raining
          (Rendering|Material|SetScalarParameterValue _material_instance_4 "Cloud opacity" (Variables|Default|GetCloudOpacity) :!class /Script/Engine.MaterialInstanceDynamic)
          (Rendering|Material|SetVectorParameterValue _material_instance_4 "Cloud color" (Variables|Components|GetCloud%20color) :!class /Script/Engine.MaterialInstanceDynamic)
          (Rendering|Material|SetScalarParameterValue _material_instance_4 "Cloud speed" (Variables|Default|GetCloudSpeed) :!class /Script/Engine.MaterialInstanceDynamic)
          (Components|Activation|SetActive (Variables|Default|GetRain) true false)
          (return)
          (elif (Utilities|Enum|Equal(Enum) (Variables|Default|GetInput) (Variables|Default|GetCloudy))
            (Variables|Default|SetCloudOpacity 6.0)
            (Variables|Components|SetCloud%20color "(R=0.610000,G=0.610000,B=0.610000,A=1.000000)")
            ;[1 1 1] Cloudy
            (Rendering|Material|SetScalarParameterValue _material_instance "Cloud opacity" (Variables|Default|GetCloudOpacity) :!class /Script/Engine.MaterialInstanceDynamic)
            (Rendering|Material|SetVectorParameterValue _material_instance "Cloud color" (Variables|Components|GetCloud%20color) :!class /Script/Engine.MaterialInstanceDynamic)
            (Rendering|Material|SetScalarParameterValue _material_instance "Cloud speed" (Variables|Default|GetCloudSpeed) :!class /Script/Engine.MaterialInstanceDynamic)
            (return)
            (elif (Utilities|Enum|Equal(Enum) (Variables|Default|GetInput) (Variables|Default|GetPartlyCloud))
              (Variables|Default|SetCloudOpacity 1.5)
              (Variables|Components|SetCloud%20color "(R=1.000000,G=1.000000,B=1.000000,A=1.000000)")
              ;[1 1 1] Partly Cloud
              (Rendering|Material|SetScalarParameterValue _material_instance_2 "Cloud opacity" (Variables|Default|GetCloudOpacity) :!class /Script/Engine.MaterialInstanceDynamic)
              (Rendering|Material|SetVectorParameterValue _material_instance_2 "Cloud color" (Variables|Components|GetCloud%20color) :!class /Script/Engine.MaterialInstanceDynamic)
              (Rendering|Material|SetScalarParameterValue _material_instance_2 "Cloud speed" (Variables|Default|GetCloudSpeed) :!class /Script/Engine.MaterialInstanceDynamic)
              (return)
              (else
                (Development|PrintString (Variables|Default|GetInput))
                (return)))))))))

(fn PlayAudio
  (params (Audio :type String))
  (if (Utilities|Enum|Equal(Enum) Audio "Sun")
    (bind _returnvalue (AddComponent|AddAudioComponent false))
    (Audio|Components|Audio|Play _returnvalue 0.0)
    (return)
    (elif (Utilities|Enum|Equal(Enum) Audio "Rain")
      (bind _returnvalue_2 (AddComponent|AddAudioComponent false))
      (Audio|Components|Audio|Play _returnvalue_2 0.0)
      (return)
      (else
        (bind _returnvalue_3 (AddComponent|AddAudioComponent false))
        (Audio|Components|Audio|Play _returnvalue_3 0.0)
        (return)))))

(fn StopAllAudio
  (bind _returnvalue (AddComponent|AddAudioComponent false))
  (bind _returnvalue_2 (AddComponent|AddAudioComponent false))
  (bind _returnvalue_3 (AddComponent|AddAudioComponent false))
  (Audio|Components|Audio|Stop _returnvalue)
  (return))