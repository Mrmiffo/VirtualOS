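; Manager actor for the virtual OS file system that spawns and closes file display windows as folders are opened and closed.
; Opening a folder offsets the root folder and existing windows by a separation vector, then spawns, initializes and displays a new window at the manager's transform.
; Closing finds the window by its root folder, removes it, and shifts windows later in the list and the root folder back.
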(event EventDisplayFiles
  (params (DisplayFolderContent :type Array%20of%20BP%20File%20Object%20References) (RootFolderOfContent :type BP%20File%20Object%20Reference))
  (CallFunction|DisplayFolderContent DisplayFolderContent RootFolderOfContent))

(event EventOpenwithRoot
  (params (PathToRootFolder :type String))
  (CallFunction|StartManager))

(event EventCloseFolder
  (params (FolderToClose :type BP%20File%20Object%20Reference))
  (CallFunction|FindandCloseDisplaybyRootFolder FolderToClose))

(fn ConstructionScript)

(fn DisplayFolderContent
  (params (FilesToDisplay :type Array%20of%20BP%20File%20Object%20References) (RootFolderOfContent :type BP%20File%20Object%20Reference))
  ;[1 1 1] Move old windows when opening new folder
  (Transformation|AddActorLocalOffset (Variables|Default|GetRootFolder) (Variables|Default|GetWindowSeperation) false false)
  (for _array_element (Variables|Default|GetWindows)
    (Transformation|AddActorLocalOffset _array_element (Variables|Default|GetWindowSeperation) false false))
  (bind _returnvalue (Game|SpawnActorfromClass "/Game/VirtualOSContent/FileSystem/Blueprints/BP_FileDisplayWindow.BP_FileDisplayWindow_C" (Transformation|GetWorldTransform (Variables|Default|GetDefaultSceneRoot)) "Undefined" 0 0))
  (Utilities|FlowControl|Sequence
    (:then_0
      (Default|Initialize _returnvalue self RootFolderOfContent FilesToDisplay))
    (:then_1
      (Utilities|Array|Add (Variables|Default|GetWindows) _returnvalue))
    (:then_2
      (Default|DisplayContent _returnvalue))))

(fn FindandCloseDisplaybyRootFolder
  (params (RootFolder :type BP%20File%20Object%20Reference))
  (bind _windowseperation (Variables|Default|GetWindowSeperation))
  (bind _returnvalue (* _windowseperation -1))
  (for _array_element (Variables|Default|GetWindows)
    ;[1 1 1] Check if it's the right window
    (if (== (Variables|/Game/VirtualOSContent/FileSystem/Blueprints/BP_FileDisplayWindow.BP_FileDisplayWindow_C|GetRootFolder _array_element) RootFolder)
      (Default|CloseDisplay _array_element)
      (LocalVariables|SetDisplayClosed true)
      (Utilities|Array|RemoveItem (Variables|Default|GetWindows) _array_element)
      (elif (LocalVariables|GetDisplayClosed)
        (Transformation|AddActorLocalOffset _array_element _returnvalue false false))))
  (if (LocalVariables|GetDisplayClosed)
    (Transformation|AddActorLocalOffset (Variables|Default|GetRootFolder) _returnvalue false false)))

(fn StartManager
  (params (RootFolder :type BP%20File%20Object%20Reference))
  (bind _output_get (Variables|Default|SetRootFolder RootFolder))
  (Transformation|AttachActorToActor _output_get self "None" "KeepWorld" "KeepWorld" "KeepWorld" true))