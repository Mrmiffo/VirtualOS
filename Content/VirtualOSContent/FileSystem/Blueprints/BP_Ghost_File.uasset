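; BP_Ghost_File is a semi-transparent file actor that is grabbed and dropped to indicate move, copy or shortcut operations in the virtual OS.
; On release, the overlapping file window and alt button pick the operation, which also drives the hint text, but operations only print placeholders.
; Window drops destroy the ghost, throws simulate physics before destroying it, and other drops just detach.
; Interacting with a directory opens it in its displaying or newly spawned window.
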(event EventBeginPlay
  (|CallParentFunction))

(event EventStartGrab
  (params (GrabbingController :type Motion%20Controller%20Component%20Object%20Reference))
  ;[1 1 1] Grab
  (bind _output_get (Variables|Default|SetGrabbingController GrabbingController))
  (Transformation|AttachComponentToComponent (Variables|Default|GetDefaultSceneRoot) _output_get "None" "KeepWorld" "KeepWorld" "KeepWorld" true))

(event EventInteract
  (params (AltButtonPressed :type Boolean))
  (bind _defaultsceneroot (Variables|Default|GetDefaultSceneRoot))
  (bind _returnvalue (Transformation|GetWorldTransform _defaultsceneroot))
  (bind (_location _rotation _scale) (Math|Transform|BreakTransform _returnvalue))
  (if (Variables|Default|GetIsDirectory)
    (Utilities|IsValid (Variables|Default|GetDisplayedBy)
      (:Is%20Valid
        (Default|OpenFolder (Variables|Default|GetDisplayedBy) (Variables|Default|GetPath)))
      (:Is%20Not%20Valid
        (bind _returnvalue_2 (Game|SpawnActorfromClass "/Game/VirtualOSContent/FileSystem/Blueprints/BP_FileDisplayWindow.BP_FileDisplayWindow_C" (Math|Transform|MakeTransform (+ (* (Math|Vector|GetForwardVector _rotation) -15) _location) _rotation _scale) "Undefined" 0 0))
        (bind _output_get (Variables|Default|SetDisplayedBy _returnvalue_2))
        (Default|OnStartup _output_get (Variables|Default|GetPath))))))

(event EventEndGrab
  (params (ReleasingController :type Motion%20Controller%20Component%20Object%20Reference) (AltButtonPressed :type Boolean) (Thrown :type Boolean))
  ;[1 1 1] Release
  (if (== ReleasingController (Variables|Default|GetGrabbingController))
    (bind _overlapped_window (CallFunction|GetOverlappingWindow))
    (Utilities|IsValid _overlapped_window
      (:Is%20Valid
        (if (== _overlapped_window (Variables|Default|GetDisplayedBy))
          (Development|PrintString "Same window, do nothing" true true "(R=0.000000,G=0.660000,B=1.000000,A=1.000000)" 4e+01)
          (elif AltButtonPressed
            (Development|PrintString "Other window, copy to window" true true "(R=0.000000,G=0.660000,B=1.000000,A=1.000000)" 4e+01)
            (else
              (Development|PrintString "Other window, move to window" true true "(R=0.000000,G=0.660000,B=1.000000,A=1.000000)" 4e+01))))
        (Actor|DestroyActor))
      (:Is%20Not%20Valid
        (if Thrown
          (Physics|SetSimulatePhysics (Variables|Default|GetFileModel) true)
          (Transformation|DetachFromActor "KeepWorld" "KeepWorld" "KeepWorld")
          (Development|PrintString "Thrown" true true "(R=0.000000,G=0.660000,B=1.000000,A=1.000000)" 4e+01)
          (Utilities|FlowControl|Delay 2.0)
          (Actor|DestroyActor)
          (else
            (Transformation|DetachFromActor "KeepWorld" "KeepWorld" "KeepWorld")
            (Development|PrintString "Create shortcut" true true "(R=0.000000,G=0.660000,B=1.000000,A=1.000000)" 4e+01)))))))

(fn ConstructionScript
  (|CallParentFunction))

(fn SetupFile
  (params (Path :type String) (Display :type BP%20File%20Display%20Window%20Object%20Reference))
  (|CallParentFunction Path Display)
  (Rendering|Material|SetScalarParameterValue (Variables|Default|GetMaterial) "Opacity" 0.7 :!class /Script/Engine.MaterialInstanceDynamic)
  (return))

(fn GetHint
  (params (AltButtonPressed :type Boolean))
  ;[1 1 1] Check if grabbed
  (if (Utilities|IsValid (Variables|Default|GetGrabbingController))
    ;[1 1 1] Create shortcut if not droped in a window
    (bind _overlapped_window (CallFunction|GetOverlappingWindow))
    (if (Utilities|IsValid _overlapped_window)
      ;[1 1 1] Copy on advanced, else move
      (if AltButtonPressed
        (return (Utilities|String|Append "Copy to" (Variables|/Game/VirtualOSContent/FileSystem/Blueprints/BP_FileDisplayWindow.BP_FileDisplayWindow_C|GetWindowName _overlapped_window)))
        (else
          (return (Utilities|String|Append "Move to " (Variables|/Game/VirtualOSContent/FileSystem/Blueprints/BP_FileDisplayWindow.BP_FileDisplayWindow_C|GetWindowName _overlapped_window)))))
      (else
        (return "Create shortcut")))
    (else
      ;[1 1 1] If not grabed, use parent hint
      (bind _hinttext (|CallParentFunction AltButtonPressed))
      (return _hinttext))))

(fn GetOverlappingWindow
  (for _array_element (Collision|GetOverlappingActors (Variables|Default|GetFileModel) "/Game/VirtualOSContent/FileSystem/Blueprints/BP_FileDisplayWindow.BP_FileDisplayWindow_C" :!class /Script/Engine.PrimitiveComponent)
    (bind _asbp_file_display_window (Utilities|Casting|CastToBP_FileDisplayWindow _array_element))
    (return _asbp_file_display_window))
  (return 0))

(fn IsRunning
  (return false))