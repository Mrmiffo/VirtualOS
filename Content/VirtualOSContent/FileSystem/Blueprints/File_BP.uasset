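; File_BP is an actor representing a file or folder in a virtual OS, which can be grabbed, docked, fetched and retreated.
; SetupFile derives the wrapped label from the path and treats dotless paths as directories, though both types use the folder mesh.
; Interacting toggles directories only: opening spawns File_BPs from a JoyFileIO listing for DisplayedBy to show, closing delegates to DisplayedBy, and material emission marks the state.
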(event EventInteract
  (bind _material (Variables|Default|GetMaterial))
  (bind _isdirectory (Variables|FileProperties|GetIsDirectory))
  ;[1 1 1] Interact - Open/Close file
  (if (Variables|Fileproperties|GetFileIsOpen)
    (if _isdirectory
      (CloseFolder|CloseFolder)
      (Variables|Fileproperties|SetFileIsOpen false)
      (Rendering|Material|SetScalarParameterValue _material "EmissionStrength" 0.0 :!class /Script/Engine.MaterialInstanceDynamic))
    (elif _isdirectory
      (OpenFolder|OpenFolder)
      (Variables|Fileproperties|SetFileIsOpen true)
      (Rendering|Material|SetScalarParameterValue _material "EmissionStrength" 2.0 :!class /Script/Engine.MaterialInstanceDynamic))))

(event EventBeginPlay
  ;[1 1 1] Start listening to input from player on spawn
  (Input|EnableInput (Game|GetPlayerController 0)))

(event EventDocked
  (params (DockedTo :type I%20Dock%20Interface))
  ;[1 1 1] Dock
  (Variables|Docking|SetObjectIsDockedTo DockedTo)
  (Variables|Docking|SetObjectIsDocked true))

(event EventUndocked
  (params (UndockedFrom :type I%20Dock%20Interface))
  ;[1 1 1] Dock
  (Variables|Docking|SetObjectIsDockedTo 0)
  (Variables|Docking|SetObjectIsDocked false))

(event EventStartGrab
  (params (GrabbingController :type Motion%20Controller%20Component%20Object%20Reference))
  ;[1 1 1] Grab
  (Transformation|AttachComponentToComponent (VehicleSound|GetRootComponent) GrabbingController "None" "KeepWorld" "KeepWorld" "KeepWorld" true))

(event EventEndGrab
  (params (ReleasingController :type Motion%20Controller%20Component%20Object%20Reference))
  ;[1 1 1] Grab
  (Transformation|DetachFromComponent (VehicleSound|GetRootComponent) "KeepRelative" "KeepRelative" "KeepRelative" true))

(event EventFetch
  (Variables|Fetch|SetRetreatLocation (Transformation|GetWorldTransform (Variables|Default|GetFileNameRenderer self)))
  (Variables|Fetch|SetHasBeenFetched true))

(event EventRetreat
  (if (Variables|Fetch|GetHasBeenFetched)
    (Transformation|SetWorldTransform (Variables|Default|GetDefaultSceneRoot) (Variables|Fetch|GetRetreatLocation) false false)))

(fn ConstructionScript
  (Setup|SetupFile (Variables|FileProperties|GetPath))
  (bind _returnvalue (Rendering|Material|CreateDynamicMaterialInstance (Rendering|Material|GetMaterial (Variables|Default|GetFileModel) 0) :!class /Script/Engine.KismetMaterialLibrary))
  (Variables|Default|SetMaterial _returnvalue))

(fn SpawnFile
  (params (Path :type String) (Name :type String))
  (bind _returnvalue (Game|SpawnActorfromClass "File_BP_C" (Transformation|GetWorldTransform (Variables|Default|GetDefaultSceneRoot)) "Undefined" 0 0))
  (bind _finalized_file (Setup|SetupFile _returnvalue Path (Variables|Default|GetDisplayedBy)))
  (return _finalized_file))

(fn SpawnFilesandFolders
  (params (Files :type Array%20of%20Strings))
  (bind _filesandfolders (LocalVariables|GetFilesAndFolders))
  (for _array_element Files
    (bind _newfile (OpenFolder|SpawnFile _array_element))
    (Utilities|Array|Add _filesandfolders _newfile))
  (return _filesandfolders))

(fn AddBreakLinetoString
  (params (LineLength :type Integer) (String :type String))
  (bind _breaklinearray (LocalVariables|GetBreakLineArray))
  (for _index (range 0 (/ (Utilities|String|Len String) LineLength))
    ;[1 1 1] Add break by splitting into array and merging with seperating <br>
    (Utilities|Array|Add _breaklinearray (Utilities|String|GetSubstring String (* _index LineLength) LineLength)))
  (return (Utilities|String|JoinStringArray _breaklinearray "<br>")))

(fn CloseFolder
  (Default|CloseFolder (Variables|Default|GetDisplayedBy) self))

(fn SetName
  (params (NewName :type String))
  (bind _filenamerenderer (Variables|Default|GetFileNameRenderer))
  (bind _linelength (LocalVariables|GetLineLength))
  (bind _output_get (Variables|FileProperties|SetName NewName))
  (if (> (Utilities|String|Len _output_get) _linelength)
    (bind _stringwithbreak (OpenFolder|AddBreakLinetoString _linelength _output_get))
    (Rendering|Components|TextRender|SetText _filenamerenderer (Utilities|Text|ToText(String) _stringwithbreak))
    (else
      (Rendering|Components|TextRender|SetText _filenamerenderer (Utilities|Text|ToText(String) (Variables|FileProperties|GetName))))))

(fn OpenFolder
  (bind _spawnedfileobjects (OpenFolder|SpawnFilesandFolders (.Files (Class|VictoryBPFunctionLibrary|JoyFileIOGetFilesinRootandAllSubFolders (Variables|FileProperties|GetPath)))))
  (Default|DisplayFiles (Variables|Default|GetDisplayedBy) _spawnedfileobjects self))

(fn SetupFile
  (params (Path :type String) (Display :type I%20File%20System%20Manager%20Interface))
  (bind _returnvalue (Utilities|String|ParseIntoArray Path "/"))
  (bind _filemodel (Variables|Default|GetFileModel))
  (Variables|Default|SetDisplayedBy Display)
  (Setup|SetName (Utilities|Array|Get(acopy) _returnvalue (Utilities|Array|LastIndex _returnvalue)))
  (bind _output_get (Variables|FileProperties|SetPath Path))
  (if (> (Utilities|Array|Length (Utilities|String|ParseIntoArray _output_get ".")) 1)
    (Variables|FileProperties|SetSuffix (Utilities|Array|Get(acopy) (Utilities|String|ParseIntoArray _output_get ".") (Utilities|Array|LastIndex (Utilities|String|ParseIntoArray _output_get "."))))
    (Variables|FileProperties|SetIsDirectory false)
    (Components|StaticMesh|SetStaticMesh _filemodel "/Game/VirtualOSContent/FileSystem/Models/folder_model.folder_model")
    (else
      (Variables|FileProperties|SetIsDirectory true)
      (Components|StaticMesh|SetStaticMesh _filemodel "/Game/VirtualOSContent/FileSystem/Models/folder_model.folder_model")))
  (return self))

(fn Dockedto
  (return (Variables|Docking|GetObjectIsDockedTo)))

(fn GetActorComponet
  (return self))

(fn IsDocked
  (return (Variables|Docking|GetObjectIsDocked)))