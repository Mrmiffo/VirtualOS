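; Virtual OS file browser manager that shows folder contents as a series of spawned, attached display windows.
; StartManager spawns a root File_BP from a path, initially a hard-coded desktop path on BeginPlay, and passes itself as its display.
; Opening a folder shifts the root and existing windows by WindowSeperation, then spawns a new FileDisplayWindow.
; Closing finds windows by root folder and shifts later entries and the root back.
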(event EventDisplayFiles
  (params (DisplayFolderContent :type Array%20of%20File%20BP%20Object%20References) (RootFolderOfContent :type File%20BP%20Object%20Reference))
  (CallFunction|DisplayFolderContent DisplayFolderContent RootFolderOfContent))

(event EventOpenwithRoot
  (params (PathToRootFolder :type String))
  (CallFunction|StartManager PathToRootFolder))

(event EventBeginPlay
  (CallFunction|StartManager "C:/Users/anton/Desktop/"))

(event EventCloseFolder
  (params (FolderToClose :type File%20BP%20Object%20Reference))
  (CallFunction|FindandCloseDisplaybyRootFolder FolderToClose))

(fn ConstructionScript)

(fn DisplayFolderContent
  (params (FilesToDisplay :type Array%20of%20File%20BP%20Object%20References) (RootFolderOfContent :type File%20BP%20Object%20Reference))
  ;[1 1 1] Move old content when opening new folder
  (Transformation|AddActorLocalOffset (Variables|Default|GetRootFolder) (Variables|Default|GetWindowSeperation) false false)
  (for _array_element (Variables|Default|GetWindows)
    (Transformation|AddActorLocalOffset _array_element (Variables|Default|GetWindowSeperation) false false))
  (bind _returnvalue (Game|SpawnActorfromClass "/Game/VirtualOSContent/FileSystem/Blueprints/FileDisplayWindow.FileDisplayWindow_C" (Transformation|GetWorldTransform (Variables|Default|GetDefaultSceneRoot)) "Undefined" 0 0))
  (Utilities|FlowControl|Sequence
    (:then_0
      (Transformation|AttachActorToActor _returnvalue self "None" "SnapToTarget" "SnapToTarget" "SnapToTarget" true))
    (:then_1
      (Utilities|Array|Add (Variables|Default|GetWindows) _returnvalue))
    (:then_2
      (Default|DisplayContent _returnvalue FilesToDisplay RootFolderOfContent))))

(fn FindandCloseDisplaybyRootFolder
  (params (RootFolder :type File%20BP%20Object%20Reference))
  (bind _windowseperation (Variables|Default|GetWindowSeperation))
  (bind _returnvalue (* _windowseperation -1))
  (for _array_element (Variables|Default|GetWindows)
    (if (== (Variables|/Game/VirtualOSContent/FileSystem/Blueprints/FileDisplayWindow.FileDisplayWindow_C|GetRootFolder _array_element) RootFolder)
      (Default|CloseDisplay _array_element)
      (LocalVariables|SetDisplayClosed true)
      (elif (LocalVariables|GetDisplayClosed)
        (Transformation|AddActorLocalOffset _array_element _returnvalue false false))))
  (if (LocalVariables|GetDisplayClosed)
    (Transformation|AddActorLocalOffset (Variables|Default|GetRootFolder) _returnvalue false false)))

(fn StartManager
  (params (RootFolder :type String))
  (bind _returnvalue (Game|SpawnActorfromClass "/Game/VirtualOSContent/FileSystem/Blueprints/File_BP.File_BP_C" (Transformation|GetWorldTransform (Variables|Default|GetDefaultSceneRoot)) "Undefined" 0 0))
  (bind _finalized_file (Default|SetupFile _returnvalue RootFolder self))
  (bind _output_get (Variables|Default|SetRootFolder _finalized_file))
  (Transformation|AttachActorToActor _output_get self "None" "SnapToTarget" "SnapToTarget" "SnapToTarget" true))