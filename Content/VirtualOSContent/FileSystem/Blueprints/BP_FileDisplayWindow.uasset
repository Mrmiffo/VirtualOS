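; File Explorer window actor for a virtual OS, showing a folder's contents as BP_File actors that can be grabbed as a window or thrown away to close.
; OpenFolder feeds Display, which builds breadcrumb tabs from the path, page buttons and a paged Snapgrid of files.
; Touch swipes and button presses change pages.
; Lerp helpers animate tabs and shrink the grid; their completion callback repopulates and regrows it.
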(event EventKill
  ;[1 1 1] Close the window, kill all content
  (for _array_element (Variables|DisplayArea|GetDisplayedContent)
    (Utilities|IsValid _array_element
      (:Is%20Valid
        (Default|Kill _array_element))))
  (for _array_element_2 (Variables|Breadcrumbs|GetBreadcrumb)
    (Utilities|IsValid _array_element_2
      (:Is%20Valid
        (Default|Kill _array_element_2))))
  (Default|Kill (Variables|DisplayArea|GetDisplayedSnapGrid))
  (CallFunction|RemovePageButtons)
  (Actor|DestroyActor))

(event EventEndGrab
  (params (ReleasingController :type Motion%20Controller%20Component%20Object%20Reference) (AltButtonPressed :type Boolean) (Thrown :type Boolean))
  ;[1 1 1] Handle Grabbing of the window
  (if (== ReleasingController (Variables|Default|GetGrabbingController))
    (if Thrown
      (Transformation|DetachFromActor "KeepWorld" "KeepWorld" "KeepWorld")
      (Physics|SetSimulatePhysics (Variables|Default|GetStaticMesh) true)
      (Utilities|FlowControl|Delay 2.0)
      (CallFunction|Kill)
      (else
        (Transformation|DetachFromActor "KeepWorld" "KeepWorld" "KeepWorld")))))

(event EventButtonPressed
  (params (ButtonThatWasPressed :type Context%20Button%20Object%20Reference) (AltButtonPressed :type Boolean))
  (MainContentDisplay|ChangeDisplayPage (Variables|/Game/VirtualOSContent/Contextmenu/Button/ContextButton.ContextButton_C|GetID ButtonThatWasPressed)))

(event EventTick
  (params (DeltaSeconds :type Float%20%28single-precision%29))
  (bind _staticmesh (Variables|Default|GetStaticMesh))
  (bind _touchedby (Variables|Default|GetTouchedBy))
  (bind _touchpageswitchsensitivity (Variables|Default|GetTouchPageSwitchSensitivity))
  (bind _displaypage (Variables|DisplayArea|GetDisplayPage))
  (bind _returnvalue (Transformation|GetWorldTransform _touchedby))
  (bind _returnvalue_2 (Transformation|GetWorldTransform _staticmesh))
  (bind _returnvalue_3 (Class|KismetMathLibrary|ConvertTransformtoRelative _returnvalue _returnvalue_2))
  (bind _location (Math|Transform|BreakTransform _returnvalue_3))
  (Utilities|IsValid _touchedby
    (:Is%20Valid
      ;[1 1 1] Swipe left increment page
      (if (>= (- (.Z (Math|Vector|BreakVector _location)) (.Z (Math|Vector|BreakVector (Variables|Default|GetTouchLocation)))) _touchpageswitchsensitivity)
        (MainContentDisplay|ChangeDisplayPage (+ _displaypage 1))
        (Variables|Default|SetTouchLocation _location :!label _label)
        (else
          ;[1 1 1] Swipe right decrement page
          (if (<= (- (.Z (Math|Vector|BreakVector _location)) (.Z (Math|Vector|BreakVector (Variables|Default|GetTouchLocation)))) (* -1 _touchpageswitchsensitivity))
            (MainContentDisplay|ChangeDisplayPage (- _displaypage 1))
            (goto _label)))))))

(event EventLerpDoneComponent
  (params (LerpHelper :type Lerp%20Helper%20Object%20Reference) (Component :type Scene%20Component%20Object%20Reference))
  ;[1 1 1] lerp reporting
  ;;[1 1 1] Used for moving breadcrumb tabs
  (Components|DestroyComponent LerpHelper))

(event EventStartTouch
  (params (TouchingController :type Scene%20Component%20Object%20Reference))
  ;[1 1 1] Start and stop touch
  (bind _output_get (Variables|Default|SetTouchedBy TouchingController))
  (Variables|Default|SetTouchLocation (.Location (Math|Transform|BreakTransform (Class|KismetMathLibrary|ConvertTransformtoRelative (Transformation|GetWorldTransform _output_get) (Transformation|GetWorldTransform (Variables|Default|GetStaticMesh)))))))

(event EventEndTouch
  (params (TouchingController :type Scene%20Component%20Object%20Reference))
  ;[1 1 1] Start and stop touch
  (if (== TouchingController (Variables|Default|GetTouchedBy))
    (Variables|Default|SetTouchedBy 0)))

(event EventLerpDoneActor
  (params (LerpHelper :type Lerp%20Helper%20Object%20Reference) (LerpedActor :type Actor%20Object%20Reference))
  ;[1 1 1] lerp reporting
  (if (Utilities|Array|ContainsItem (Variables|DisplayArea|GetLerpRemove) LerpHelper)
    ;;[1 1 1] Clear displayed content if the object was the snapgrid, and repopulate it with new content and return it to size
    (if (== LerpedActor (Variables|DisplayArea|GetDisplayedSnapGrid))
      (MainContentDisplay|ClearDisplayedContent)
      (MainContentDisplay|SelectContenttoDisplay)
      (MainContentDisplay|AnimateResetSize (Variables|DisplayArea|GetDisplayedSnapGrid))
      (else
        ;;[1 1 1] Destroy the actor if it was not snapgrid
        (Actor|DestroyActor LerpedActor)))
    (Utilities|Array|RemoveItem (Variables|DisplayArea|GetLerpRemove) LerpHelper)
    (Components|DestroyComponent LerpHelper)
    (else
      ;;[1 1 1] Only destroy the lerper if the object was not supposed to be removed (ie only be moved)
      (Components|DestroyComponent LerpHelper))))

(event EventStartGrab
  (params (GrabbingController :type Motion%20Controller%20Component%20Object%20Reference))
  ;[1 1 1] Handle Grabbing of the window
  (bind _output_get (Variables|Default|SetGrabbingController GrabbingController))
  (Transformation|AttachComponentToComponent (Variables|Default|GetDefaultSceneRoot) _output_get "None" "KeepWorld" "KeepWorld" "KeepWorld" true))

(event EventOnStartup
  (params (startParams :type String))
  (CallFunction|OpenFolder startParams))

(fn ConstructionScript)

(fn Display
  (params (FilesToDisplay :type Array%20of%20Strings) (PathOfFolder :type String))
  (Variables|DisplayArea|SetWindowContent FilesToDisplay)
  (Variables|DisplayArea|SetDisplayPage 0)
  ;[1 0.3331 0] Set the displayed name of the window - NOT IN USE
  (bind _output_get (Variables|Breadcrumbs|SetWindowPath PathOfFolder))
  (bind _returnvalue (Class|FileSystemBPLibrary|GetCleanFileName _output_get))
  (Variables|Default|SetWindowName _returnvalue)
  (CallFunction|ManagePageButtons)
  (Breadcrumbs|ManageBreadcrumbs PathOfFolder)
  (Utilities|IsValid (Variables|DisplayArea|GetDisplayedSnapGrid)
    (:Is%20Valid
      ;[1 1 1] Select content to Display is run after animation is done from event graph
      (MainContentDisplay|AnimateRemove (Variables|DisplayArea|GetDisplayedSnapGrid)))
    (:Is%20Not%20Valid
      ;[1 1 1] Run only when the window is opened for the first time
      (MainContentDisplay|CreateSnapGrid)
      (MainContentDisplay|SelectContenttoDisplay))))

(fn ClearDisplayedContent
  (for _array_element (Variables|DisplayArea|GetDisplayedContent)
    (Actor|DestroyActor _array_element))
  (Utilities|Array|Clear (Variables|DisplayArea|GetDisplayedContent)))

(fn ManageBreadcrumbs
  (params (PathOfWindow :type String))
  (bind _breadcrumb (Variables|Breadcrumbs|GetBreadcrumb))
  ;[1 1 1] Destroy old breadcrumbs
  (for _array_element _breadcrumb
    (Utilities|IsValid _array_element
      (:Is%20Valid
        (Actor|DestroyActor _array_element))))
  (Utilities|Array|Clear _breadcrumb)
  ;[1 1 1] Create new breadcrumbs
  (for (_array_element_2 _array_index) (Utilities|String|ParseIntoArray PathOfWindow "/")
    ;;[1 1 1] If it's the first object initialize the Reconstruction path
    (if (== _array_index 0)
      (LocalVariables|SetReconstructedPath _array_element_2)
      (else
        (LocalVariables|SetReconstructedPath (Utilities|String|Append (LocalVariables|GetReconstructedPath) "/" _array_element_2))))
    ;;[1 1 1] Create breadcrumb files
    (bind _newfile (CallFunction|CreateFile (LocalVariables|GetReconstructedPath)))
    (Utilities|Array|Add (Variables|Breadcrumbs|GetBreadcrumb) _newfile))
  (Breadcrumbs|DisplayBreadcrumbs))

(fn DisplayBreadcrumbs
  (bind _breadcrumb (Variables|Breadcrumbs|GetBreadcrumb))
  (bind _displayeditems (LocalVariables|GetDisplayeditems))
  (bind (_arrayindex _arrayelement) (Utilities|Array|ReverseforEachLoop _breadcrumb)
    (:LoopBody
      (if (< (LocalVariables|GetDisplayeditems) 6)
        (Utilities|IsValid _arrayelement
          (:Is%20Valid
            (Transformation|AttachComponentToComponent _arrayelement (Utilities|Array|Get(acopy) (Actor|GetComponentsbyTag "/Script/Engine.SceneComponent" (Utilities|String|StringToName (Utilities|String|Append "Breadcrumb" (Utilities|String|ToString(Integer) (- (Utilities|Array|Length _breadcrumb) (+ _arrayindex 1))))))) "None" "SnapToTarget" "SnapToTarget" "SnapToTarget" true)
            (Math|Integer|IncrementInt (LocalVariables|GetDisplayeditems)
              (:%20%20
                (Transformation|SetActorRelativeScale3D _arrayelement (* (Class|Actor|GetActorRelativeScale3D _arrayelement) "0.400000,0.400000,0.400000"))))))
        (else
          (Utilities|IsValid _arrayelement
            (:Is%20Valid
              (Actor|DestroyActor _arrayelement))))))
    (:Completed
      ;[1 1 1] Hide unused tabs
      (Breadcrumbs|SetBreadcrumbTabVisiblity 1 (- _displayeditems 1) true)
      (Breadcrumbs|SetBreadcrumbTabVisiblity _displayeditems 5 false))))

(fn CreateFile
  (params (Path :type String))
  (bind _returnvalue (Game|SpawnActorfromClass "/Game/VirtualOSContent/FileSystem/Blueprints/BP_File.BP_File_C" (Transformation|GetWorldTransform (Variables|Default|GetDefaultSceneRoot)) "Undefined" 0 0))
  (Default|SetupFile _returnvalue Path self)
  (return _returnvalue))

(fn OpenFolder
  (params (Path :type String))
  (bind _returnvalue (Class|FileSystemBPLibrary|GetFolderContent Path))
  (MainContentDisplay|Display _returnvalue Path))

(fn CreateSnapGrid
  (bind _returnvalue (Game|SpawnActorfromClass "/Game/VirtualOSContent/Snapgrid/Snapgrid.Snapgrid_C" (Transformation|GetWorldTransform (Variables|Default|GetDefaultSceneRoot)) "Undefined" 0 0))
  (bind _output_get (Variables|DisplayArea|SetDisplayedSnapGrid _returnvalue))
  (Transformation|AttachActorToActor _output_get self "None" "SnapToTarget" "SnapToTarget" "SnapToTarget" true)
  (Transformation|AttachComponentToComponent _output_get (Variables|Default|GetFileOrigin) "None" "SnapToTarget" "SnapToTarget" "SnapToTarget" true)
  (Default|Setup _output_get (Variables|DisplayArea|GetNoOfColumns) (Variables|DisplayArea|GetNoOfRows) (Variables|DisplayArea|GetDisplayAreaWidth) (Variables|DisplayArea|GetDisplayAreaHeight) "NewEnumerator0"))

(fn SetBreadcrumbTabVisiblity
  (params (From :type Integer) (To :type Integer) (Visibility :type Boolean))
  ;[1 1 1] Hide tabs that are not is use
  (for _index (range From To)
    (Utilities|IsValid (Utilities|Array|Get(acopy) (Actor|GetComponentsbyTag "/Script/Engine.StaticMeshComponent" (Utilities|String|StringToName (Utilities|String|Append "Tab" (Utilities|String|ToString(Integer) _index)))))
      (:Is%20Valid
        (Breadcrumbs|AnimateDisplayBCTab (Utilities|Array|Get(acopy) (Actor|GetComponentsbyTag "/Script/Engine.StaticMeshComponent" (Utilities|String|StringToName (Utilities|String|Append "Tab" (Utilities|String|ToString(Integer) _index))))) Visibility)))))

(fn AnimateRemove
  (params (ActorToRemove :type Actor%20Object%20Reference))
  (bind _returnvalue (VehicleSound|GetRootComponent ActorToRemove))
  (bind _returnvalue_2 (Transformation|GetRelativeTransform _returnvalue))
  (bind (_location _rotation) (Math|Transform|BreakTransform _returnvalue_2))
  (bind _returnvalue_3 (AddComponent|AddLerpHelper false))
  (Utilities|Array|Add (Variables|DisplayArea|GetLerpRemove) _returnvalue_3)
  (Default|LerpTransformActor _returnvalue_3 0.2 (Math|Transform|MakeTransform _location _rotation "0.010000,0.010000,0.010000") ActorToRemove self))

(fn AnimateDisplayBCTab
  (params (ComponentToMove :type Scene%20Component%20Object%20Reference) (DisplayTab :type Boolean))
  (bind _returnvalue (Transformation|GetRelativeTransform ComponentToMove))
  (bind (_location _rotation _scale) (Math|Transform|BreakTransform _returnvalue))
  (bind (_x _y _z) (Math|Vector|BreakVector _location))
  (if DisplayTab
    (LocalVariables|SetNewVectorYValue (LocalVariables|GetDisplayYValue))
    (else
      (LocalVariables|SetNewVectorYValue (LocalVariables|GetHideYValue))))
  (bind _returnvalue_2 (AddComponent|AddLerpHelper false))
  (Default|LerpTransformComponent _returnvalue_2 0.2 (Math|Transform|MakeTransform (Math|Vector|MakeVector _x (LocalVariables|GetNewVectorYValue) _z) _rotation _scale) self ComponentToMove))

(fn SelectContenttoDisplay
  (bind _displaypage (Variables|DisplayArea|GetDisplayPage))
  (bind _displayedcontent (Variables|DisplayArea|GetDisplayedContent))
  (bind _windowcontent (Variables|DisplayArea|GetWindowContent))
  (bind _noofcolumns (Variables|DisplayArea|GetNoOfColumns))
  (bind _noofrows (Variables|DisplayArea|GetNoOfRows))
  (bind _returnvalue (* _noofcolumns _noofrows))
  (bind _returnvalue_2 (* _returnvalue _displaypage))
  ;[1 1 1] Reduce by 1 due to inclusive nature of ForLoop
  (for _index (range _returnvalue_2 (- (Math|Integer|Min(Integer) (Utilities|Array|Length _windowcontent) (+ _returnvalue _returnvalue_2)) 1))
    ;[1 1 1] Create files and position them in the grid
    (bind _newfile (CallFunction|CreateFile (Utilities|Array|Get(acopy) _windowcontent _index)))
    (Utilities|Array|Add _displayedcontent _newfile))
  (Default|AttachList (Variables|DisplayArea|GetDisplayedSnapGrid) _displayedcontent)
  (for (_array_element _array_index) (Variables|Default|GetPageButtons)
    (if (== _array_index (Variables|DisplayArea|GetDisplayPage))
      (Default|ChangeMaterial _array_element "/Game/VirtualOSContent/Thermometer/IndicatorMat.IndicatorMat")
      (else
        (Default|ChangeMaterial _array_element "/Game/VirtualOSContent/ImageViewer/blankMaterial.blankMaterial")))))

(fn AnimateResetSize
  (params (ToTransform :type Actor%20Object%20Reference))
  (bind _returnvalue (VehicleSound|GetRootComponent ToTransform))
  (bind _returnvalue_2 (Transformation|GetRelativeTransform _returnvalue))
  (bind (_location _rotation) (Math|Transform|BreakTransform _returnvalue_2))
  (bind _returnvalue_3 (AddComponent|AddLerpHelper false))
  (Default|LerpTransformActor _returnvalue_3 0.2 (Math|Transform|MakeTransform _location _rotation) ToTransform self))

(fn ChangeDisplayPage
  (params (RequestedPage :type Integer))
  (if (Math|Boolean|ANDBoolean (>= RequestedPage 0) (< (* RequestedPage (Variables|DisplayArea|GetNoOfColumns) (Variables|DisplayArea|GetNoOfRows)) (Utilities|Array|Length (Variables|DisplayArea|GetWindowContent))) (!= RequestedPage (Variables|DisplayArea|GetDisplayPage)))
    ;[1 1 1] Select items to display is called automatically in event graph
    (Variables|DisplayArea|SetDisplayPage RequestedPage)
    (MainContentDisplay|AnimateRemove (Variables|DisplayArea|GetDisplayedSnapGrid))))

(fn ManagePageButtons
  (bind _windowcontent (Variables|DisplayArea|GetWindowContent))
  (bind _noofcolumns (Variables|DisplayArea|GetNoOfColumns))
  (bind _noofrows (Variables|DisplayArea|GetNoOfRows))
  (bind _returnvalue (Utilities|Array|Length _windowcontent))
  (bind _returnvalue_2 (* _noofcolumns _noofrows))
  (bind _returnvalue_3 (Math|Conversions|ToFloat(Integer) _returnvalue))
  (bind _returnvalue_4 (Math|Conversions|ToFloat(Integer) _returnvalue_2))
  (bind _returnvalue_5 (/ _returnvalue_3 _returnvalue_4))
  (bind _returnvalue_6 (Math|Float|Ceil _returnvalue_5))
  (CallFunction|RemovePageButtons)
  (bind _returnvalue_7 (Game|SpawnActorfromClass "/Game/VirtualOSContent/Snapgrid/Snapgrid.Snapgrid_C" (Transformation|GetWorldTransform (Variables|Default|GetButtonStart)) "Undefined" 0 0))
  (Transformation|AttachComponentToComponent _returnvalue_7 (Variables|Default|GetButtonStart) "None" "SnapToTarget" "SnapToTarget" "KeepWorld" true)
  (Variables|Default|SetButtonSnapgrid _returnvalue_7)
  (Default|Setup _returnvalue_7 _returnvalue_6 1 (Math|Conversions|ToFloat(Integer) (* _returnvalue_6 12)) 2.0 "NewEnumerator0")
  (for _index (range 0 (- _returnvalue_6 1))
    (bind _returnvalue_8 (Game|SpawnActorfromClass "/Game/VirtualOSContent/Contextmenu/Button/ContextButton.ContextButton_C" (Transformation|GetWorldTransform (Variables|Default|GetButtonStart)) "Undefined" 0 0))
    (Default|Setup _returnvalue_8 "/Game/VirtualOSContent/ImageViewer/blankMaterial.blankMaterial" "PageButton" _index "" self "3.000000,3.000000,3.000000")
    (Utilities|Array|Add (Variables|Default|GetPageButtons) _returnvalue_8))
  (Default|AttachList _returnvalue_7 (Variables|Default|GetPageButtons)))

(fn RemovePageButtons
  (bind _pagebuttons (Variables|Default|GetPageButtons))
  (bind _buttonsnapgrid (Variables|Default|GetButtonSnapgrid))
  (for _array_element _pagebuttons
    (Default|Kill _array_element))
  (Utilities|Array|Clear _pagebuttons)
  (Utilities|IsValid _buttonsnapgrid
    (:Is%20Valid
      (Default|Kill _buttonsnapgrid))))

(fn GetProgramHologram
  (return "/Game/VirtualOSContent/FileSystem/Models/folder_model.folder_model"))

(fn GetProgramName
  (return "File Explorer"))

(fn IsRunning
  (return false))