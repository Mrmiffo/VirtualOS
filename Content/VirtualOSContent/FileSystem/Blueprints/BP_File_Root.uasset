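; Base file actor for the virtual OS file system, representing a file that can be grabbed and moved by a controller.
; SetupFile spawns a display window manager at the file's transform, starts it with this file and makes the material semi-transparent.
; Grabbing attaches the root to the controller, and a matching release re-attaches the file to another actor, both keeping world transform.
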(event EventBeginPlay
  (|CallParentFunction))

(event Collision|EventActorBeginOverlap
  (params (OtherActor :type Actor%20Object%20Reference)))

(event EventTick
  (params (DeltaSeconds :type Float%20%28single-precision%29)))

(event EventStartGrab
  (params (GrabbingController :type Motion%20Controller%20Component%20Object%20Reference))
  (bind _output_get (Variables|Default|SetGrabbingController GrabbingController))
  (Transformation|AttachComponentToComponent (Variables|Default|GetDefaultSceneRoot) _output_get "None" "KeepWorld" "KeepWorld" "KeepWorld" true))

(event EventEndGrab
  (if (== 0 (Variables|Default|GetGrabbingController))
    (bind _asactor (Utilities|Casting|CastToActor 0))
    (Transformation|AttachActorToActor _asactor "None" "KeepWorld" "KeepWorld" "KeepWorld" true)))

(fn ConstructionScript
  (|CallParentFunction))

(fn SetupFile
  (bind _returnvalue (Game|SpawnActorfromClass "/Game/VirtualOSContent/FileSystem/Blueprints/BP_FileDisplayWindowManager.BP_FileDisplayWindowManager_C" (Transformation|GetWorldTransform (Variables|Default|GetDefaultSceneRoot)) "Undefined" 0 0))
  (Default|StartManager _returnvalue self)
  (Rendering|Material|SetScalarParameterValue (Variables|Default|GetMaterial) "Opacity" 0.7 :!class /Script/Engine.MaterialInstanceDynamic)
  (return))