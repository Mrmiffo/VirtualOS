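; A file browser window Actor for the virtual OS file system that displays a root folder's contents as Actors in the world.
; DisplayContent stores the items, lays them out in a grid from FirstFileLocation, wrapping by NoOfLines, and attaches them to that component.
; Each Tick, only items overlapping DisplayArea stay visible, so that component acts as a clipping region.
; CloseDisplay destroys every displayed item and then the window itself.
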(event EventTick
  (params (DeltaSeconds :type Float%20%28single-precision%29))
  ;[1 1 1] Setting visibility of files
  (for _array_element (Variables|Default|GetDisplayedContent)
    (Rendering|SetVisibility (Variables|/Game/VirtualOSContent/FileSystem/Blueprints/File_BP.File_BP_C|GetDefaultSceneRoot _array_element) (Collision|IsOverlappingActor (Variables|Default|GetDisplayArea) _array_element :!class /Script/Engine.PrimitiveComponent) true)))

(event EventDisplayContent
  (params (ContentToDisplay :type Array%20of%20File%20BP%20Object%20References) (RootFolder :type File%20BP%20Object%20Reference))
  (bind _nooflines (Variables|Default|GetNoOfLines))
  (Variables|Default|SetRootFolder RootFolder)
  (bind _output_get (Variables|Default|SetDisplayedContent ContentToDisplay))
  (for (_array_element _array_index) _output_get
    ;[1 1 1] Set location
    (Transformation|SetWorldLocation (Variables|/Game/VirtualOSContent/FileSystem/Blueprints/File_BP.File_BP_C|GetDefaultSceneRoot _array_element) (+ (Math|Vector|MakeVector 0.0 (* (/ _array_index _nooflines) (Variables|Default|GetNextObjectDistance)) (* (Math|Integer|%(Integer) _array_index _nooflines) (Variables|Default|GetNewLineDistance))) (Transformation|GetWorldLocation (Variables|Default|GetFirstFileLocation))) true false)
    (Transformation|AttachComponentToComponent (Variables|/Game/VirtualOSContent/FileSystem/Blueprints/File_BP.File_BP_C|GetDefaultSceneRoot _array_element) (Variables|Default|GetFirstFileLocation) "None" "KeepWorld" "KeepWorld" "KeepWorld" true)))

(event EventCloseDisplay
  (for _array_element (Variables|Default|GetDisplayedContent)
    (Actor|DestroyActor _array_element))
  (Actor|DestroyActor))

(fn ConstructionScript)