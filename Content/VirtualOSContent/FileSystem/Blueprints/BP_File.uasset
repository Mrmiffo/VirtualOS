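; BP_File is an interactable 3D representation of a file or folder in a virtual file system.
; SetupFile derives a wrapped name label from the path and picks a folder, generic or image mesh, loading image files as textures.
; Interacting toggles folders through the owning display with an emissive highlight, while grabbing hands off to a new root that display creates.
; It also tracks docking and supports fetch and retreat.
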(event EventInteract
  (bind _self self)
  (bind _material (Variables|Default|GetMaterial))
  (bind _displayedby (Variables|Default|GetDisplayedBy))
  (bind _isdirectory (Variables|FileProperties|GetIsDirectory))
  ;[1 1 1] Interact - Open/Close file
  (if (Variables|Fileproperties|GetFileIsOpen)
    (if _isdirectory
      (Default|CloseFolder _displayedby _self)
      (Variables|Fileproperties|SetFileIsOpen false)
      (Rendering|Material|SetScalarParameterValue _material "EmissionStrength" 0.0 :!class /Script/Engine.MaterialInstanceDynamic))
    (elif _isdirectory
      (Default|OpenFolder _displayedby _self)
      (Variables|Fileproperties|SetFileIsOpen true)
      (Rendering|Material|SetScalarParameterValue _material "EmissionStrength" 2.0 :!class /Script/Engine.MaterialInstanceDynamic))))

(event EventBeginPlay
  ;[1 1 1] Start listening to input from player on spawn
  (Input|EnableInput (Game|GetPlayerController 0)))

(event EventDocked
  (params (DockedTo :type I%20Dock%20Interface))
  ;[1 1 1] Dock
  (Variables|Docking|SetObjectIsDockedTo DockedTo)
  (Variables|Docking|SetObjectIsDocked true))

(event EventUndocked
  (params (UndockedFrom :type I%20Dock%20Interface))
  ;[1 1 1] Dock
  (Variables|Docking|SetObjectIsDockedTo 0)
  (Variables|Docking|SetObjectIsDocked false))

(event EventStartGrab
  (params (GrabbingController :type Motion%20Controller%20Component%20Object%20Reference))
  ;[1 1 1] Grab
  (bind _newrootfile (Default|CreateNewRoot (Variables|Default|GetDisplayedBy) (Variables|FileProperties|GetPath)))
  (CallFunction|StartGrab _newrootfile GrabbingController))

(event EventEndGrab
  (params (ReleasingController :type Motion%20Controller%20Component%20Object%20Reference))
  ;[1 1 1] Grab
  (CallFunction|EndGrab (stale EventStartGrab _newrootfile) ReleasingController))

(event EventFetch
  ;[1 1 1] Fetch
  (Variables|Fetch|SetRetreatLocation (Transformation|GetWorldTransform (Variables|Default|GetFileNameRenderer self)))
  (Variables|Fetch|SetHasBeenFetched true))

(event EventRetreat
  ;[1 1 1] Fetch
  (if (Variables|Fetch|GetHasBeenFetched)
    (Transformation|SetWorldTransform (Variables|Default|GetDefaultSceneRoot) (Variables|Fetch|GetRetreatLocation) false false)))

(fn ConstructionScript)

(fn AddBreakLinetoString
  (params (LineLength :type Integer) (String :type String))
  (bind _breaklinearray (LocalVariables|GetBreakLineArray))
  (for _index (range 0 (/ (Utilities|String|Len String) LineLength))
    ;[1 1 1] Add break by splitting into array and merging with seperating <br>
    (Utilities|Array|Add _breaklinearray (Utilities|String|GetSubstring String (* _index LineLength) LineLength)))
  (return (Utilities|String|JoinStringArray _breaklinearray "<br>")))

(fn SetName
  (params (NewName :type String))
  (bind _filenamerenderer (Variables|Default|GetFileNameRenderer))
  (bind _linelength (LocalVariables|GetLineLength))
  (bind _output_get (Variables|FileProperties|SetName NewName))
  (if (> (Utilities|String|Len _output_get) _linelength)
    (bind _stringwithbreak (Setup|AddBreakLinetoString _linelength _output_get))
    (Rendering|Components|TextRender|SetText _filenamerenderer (Utilities|Text|ToText(String) _stringwithbreak))
    (else
      (Rendering|Components|TextRender|SetText _filenamerenderer (Utilities|Text|ToText(String) (Variables|FileProperties|GetName))))))

(fn SetupFile
  (params (Path :type String) (Display :type I%20File%20System%20Manager%20Interface))
  (bind _returnvalue (Utilities|String|ParseIntoArray Path "/"))
  (bind _filemodel (Variables|Default|GetFileModel))
  (bind _returnvalue_2 (Utilities|Array|LastIndex _returnvalue))
  (bind _item (Utilities|Array|Get(acopy) _returnvalue _returnvalue_2))
  (bind _returnvalue_3 (Utilities|String|ParseIntoArray _item "."))
  (Variables|Default|SetDisplayedBy Display)
  (Variables|FileProperties|SetPath Path)
  (Setup|SetName (Utilities|Array|Get(acopy) _returnvalue_3))
  (bind _returnvalue_4 (Class|FileSystemBPLibrary|IsDirectory Path))
  (if _returnvalue_4
    (Variables|FileProperties|SetIsDirectory true)
    ;[1 1 1] Set the corresponding mesh and make it editable
    (Components|StaticMesh|SetStaticMesh _filemodel "/Game/VirtualOSContent/FileSystem/Models/folder_model.folder_model")
    (bind _returnvalue_5 (Rendering|Material|CreateDynamicMaterialInstance _filemodel 0 "/Game/VirtualOSContent/FileSystem/Material/M_Folder.M_Folder" :!class /Script/Engine.PrimitiveComponent))
    (Variables|Default|SetMaterial _returnvalue_5)
    (else
      (Variables|FileProperties|SetSuffix (Utilities|Array|Get(acopy) _returnvalue_3 (Utilities|Array|LastIndex _returnvalue_3)))
      (Variables|FileProperties|SetIsDirectory false)
      (Setup|SetFileType)
      (switch Utilities|FlowControl|Switch|SwitchonFileType (Variables|Default|GetFileType)
        (:NewEnumerator1
          (Components|StaticMesh|SetStaticMesh _filemodel "/Game/VirtualOSContent/FileSystem/Models/fileicon.fileicon" :!label _label)
          (bind _returnvalue_6 (Rendering|Material|CreateDynamicMaterialInstance _filemodel 0 "/Game/VirtualOSContent/FileSystem/Material/M_FileIcon.M_FileIcon" :!class /Script/Engine.PrimitiveComponent))
          (Variables|Default|SetMaterial _returnvalue_6))
        (:NewEnumerator0
          (bind _success (Setup|SetImageMesh))
          (if (not _success)
            (goto _label)))))))

(fn SetFileType
  (bind _suffix (Variables|FileProperties|GetSuffix))
  (if (Math|Boolean|ORBoolean (Utilities|Enum|Equal(Enum) _suffix "png") (Utilities|Enum|Equal(Enum) _suffix "jpg") (Utilities|Enum|Equal(Enum) _suffix "bmp") (Utilities|Enum|Equal(Enum) _suffix "ico") (Utilities|Enum|Equal(Enum) _suffix "exr") (Utilities|Enum|Equal(Enum) _suffix "icns"))
    (Variables|Default|SetFileType "NewEnumerator0")
    (else
      (Variables|Default|SetFileType "NewEnumerator1"))))

(fn SetImageMesh
  (bind _filemodel (Variables|Default|GetFileModel))
  (Components|StaticMesh|SetStaticMesh _filemodel "/Game/VirtualOSContent/FileSystem/Models/ImgDisplayFile.ImgDisplayFile")
  (bind _returnvalue (Rendering|Material|CreateDynamicMaterialInstance _filemodel 0 "/Game/VirtualOSContent/FileSystem/Material/M_ImgRender.M_ImgRender" :!class /Script/Engine.PrimitiveComponent))
  (bind _output_get (Variables|Default|SetMaterial _returnvalue))
  (Rendering|Material|SetMaterial _filemodel 0 _output_get)
  (bind (_isvalid _outwidth _outheight _returnvalue_2) (Class|VictoryBPFunctionLibrary|LoadTexture2DfromFilebyExtension (Variables|FileProperties|GetPath)))
  (if _isvalid
    (Rendering|Material|SetTextureParameterValue (Variables|Default|GetMaterial) "Texture" _returnvalue_2)
    (if (== (Math|Integer|Max(Integer) _outwidth _outheight) 0)
      (return false)
      (else
        (Rendering|Material|SetScalarParameterValue (Variables|Default|GetMaterial) "ObjectScale" 0.1 :!class /Script/Engine.MaterialInstanceDynamic)
        (return true)))
    (else
      (return false))))

(fn Dockedto
  (return (Variables|Docking|GetObjectIsDockedTo)))

(fn GetActorComponet
  (return self))

(fn IsDocked
  (return (Variables|Docking|GetObjectIsDocked)))