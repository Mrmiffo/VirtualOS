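; Picture frame actor that displays an image file from disk and can be grabbed by controllers.
; DisplayPic picks the format by extension, loads it through Victory plugin into a dynamic material, and scales the mesh to keep aspect ratio, longer side matching ScaleInMeters.
; Grabbing attaches the frame to the controller.
; Release by that controller detaches it, or, if thrown, enables physics on the picture and destroys the actor after a short delay.
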(event EventBeginPlay)

(event Collision|EventActorBeginOverlap
  (params (OtherActor :type Actor%20Object%20Reference)))

(event EventStartGrab
  (params (GrabbingController :type Motion%20Controller%20Component%20Object%20Reference))
  ;[1 1 1] Grab and release
  (bind _output_get (Variables|Default|SetGrabbingController GrabbingController))
  (Transformation|AttachComponentToComponent (Variables|Default|GetDefaultSceneRoot) _output_get "None" "KeepWorld" "KeepWorld" "KeepWorld" true))

(event EventEndGrab
  (params (ReleasingController :type Motion%20Controller%20Component%20Object%20Reference) (AltButtonPressed :type Boolean) (Thrown :type Boolean))
  ;[1 1 1] Grab and release
  (if (== ReleasingController (Variables|Default|GetGrabbingController))
    (if Thrown
      (Physics|SetSimulatePhysics (Variables|Default|GetPicture) true)
      (Utilities|FlowControl|Delay 2.0)
      (Actor|DestroyActor)
      (else
        (Transformation|DetachFromActor "KeepWorld" "KeepWorld" "KeepWorld")))))

(event EventTick
  (params (DeltaSeconds :type Float%20%28single-precision%29)))

(event EventDisplayPic
  (params (Path :type String) (ScaleInMeters :type Float%20%28single-precision%29))
  (CallFunction|DisplayImage Path ScaleInMeters))

(fn ConstructionScript)

(fn GetCorrectScale
  (params (HeightInput :type Integer) (WidthInput :type Integer) (Scale :type Float%20%28single-precision%29))
  (LocalVariables|SetMaxLength Scale)
  (bind _output_get (LocalVariables|SetOldHeight HeightInput))
  (bind _output_get_2 (LocalVariables|SetOldWidth WidthInput))
  (if (>= _output_get _output_get_2)
    (LocalVariables|SetNewHeight (LocalVariables|GetMaxLength))
    (bind _calulatedwidth (CallFunction|GetNewWidth (LocalVariables|GetOldWidth) (LocalVariables|GetOldHeight) (LocalVariables|GetMaxLength)))
    (LocalVariables|SetNewWidth _calulatedwidth)
    (else
      (LocalVariables|SetNewWidth (LocalVariables|GetMaxLength))
      (bind _calculatedheight (CallFunction|GetNewHeight (LocalVariables|GetOldHeight) (LocalVariables|GetOldWidth) (LocalVariables|GetMaxLength)))
      (LocalVariables|SetNewHeight _calculatedheight)))
  (return (Math|Vector|MakeVector 0.01 (LocalVariables|GetNewWidth) (LocalVariables|GetNewHeight))))

(fn GetNewWidth
  (params (OldWidth :type Integer) (OldHeight :type Integer) (Scale :type Float%20%28single-precision%29))
  (return (* (/ (Math|Conversions|ToFloat(Integer) OldWidth) (Math|Conversions|ToFloat(Integer) OldHeight)) Scale)))

(fn GetNewHeight
  (params (OldHeight :type Integer) (OldWidth :type Integer) (Scale :type Float%20%28single-precision%29))
  (return (* (/ (Math|Conversions|ToFloat(Integer) OldHeight) (Math|Conversions|ToFloat(Integer) OldWidth)) Scale)))

(fn DisplayImage
  (params (Path :type String) (ScaleInMeters :type Float%20%28single-precision%29))
  (bind _picture (Variables|Default|GetPicture))
  (bind _fileformat (CallFunction|CheckFileExtention Path))
  (bind _returnvalue (Rendering|Material|CreateDynamicMaterialInstance "/Game/VirtualOSContent/PictureFrame/Materials/TextureMaterial.TextureMaterial" :!class /Script/Engine.KismetMaterialLibrary))
  (Rendering|Material|SetTextureParameterValue _returnvalue "Pic" (.ReturnValue (Class|VictoryBPFunctionLibrary|VictoryLoadTexture2DfromFile Path _fileformat)))
  (Rendering|Material|SetMaterial _picture 0 _returnvalue)
  (bind _picscale (CallFunction|GetCorrectScale (.Height (Class|VictoryBPFunctionLibrary|VictoryLoadTexture2DfromFile Path _fileformat)) (.Width (Class|VictoryBPFunctionLibrary|VictoryLoadTexture2DfromFile Path _fileformat)) ScaleInMeters))
  (Transformation|SetRelativeScale3D _picture _picscale))

(fn CheckFileExtention
  (params (Path :type String))
  (bind _returnvalue (Class|FileSystemBPLibrary|GetFileExtention Path))
  (switch string _returnvalue
    (:.jpg
      (LocalVariables|SetFileFormatEnum (Utilities|Enum|LiteralenumEJoyImageFormats "JPG")))
    (:.png
      (LocalVariables|SetFileFormatEnum (Utilities|Enum|LiteralenumEJoyImageFormats "PNG")))
    (:.bmp
      (LocalVariables|SetFileFormatEnum (Utilities|Enum|LiteralenumEJoyImageFormats "BMP")))
    (:.ico
      (LocalVariables|SetFileFormatEnum (Utilities|Enum|LiteralenumEJoyImageFormats "ICO")))
    (:.exr
      (LocalVariables|SetFileFormatEnum (Utilities|Enum|LiteralenumEJoyImageFormats "EXR")))
    (:.icns
      (LocalVariables|SetFileFormatEnum (Utilities|Enum|LiteralenumEJoyImageFormats "ICNS"))))
  (return (LocalVariables|GetFileFormatEnum)))