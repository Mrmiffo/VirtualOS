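; Grabbable Forecast program actor for a virtual OS that displays a five-day weather forecast and destroys itself shortly after being thrown.
; Tick, gated by a Delay, requests JSON from a URL on start and every half hour, retrying if the forecast array is missing.
; Forecast entries 1–5 (skipping 0) fill per-day text fields, with highs converted to Celsius.
; DetermineWeatherIcon maps condition text through group arrays to keys that select each day's icon material.
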(event Custom|CustomEvent
  (params (bSuccess :type Boolean) (JSON :type Json%20Field%20Data%20Object%20Reference) (Status :type EJSONResult%20Enum))
  (bind (_success _returnvalue) (Class|JsonFieldData|GetObject JSON "query"))
  (bind _returnvalue_2 (Class|JsonFieldData|GetObject _returnvalue "results"))
  (bind _returnvalue_3 (Class|JsonFieldData|GetObject _returnvalue_2 "channel"))
  (bind _returnvalue_4 (Class|JsonFieldData|GetObject _returnvalue_3 "item"))
  (bind (_success_2 _returnvalue_5) (Class|JsonFieldData|GetObjectArray _returnvalue_4 "forecast"))
  ;[1 1 1] Get weather information via JSON
  (if bSuccess
    (if _success
      (if _success_2
        ;[1 1 1] Set appropriate icon, date, day and degree to the different text fields
        (for (_array_element _array_index) _returnvalue_5
          (Variables|Default|SetText (.ReturnValue (Class|JsonFieldData|GetString _array_element "text")))
          (if (== _array_index 1)
            (bind _key (CallFunction|DetermineWeatherIcon (Variables|Default|GetText)))
            (CallFunction|Day1 (Utilities|Text|ToText(String) (.ReturnValue (Class|JsonFieldData|GetString _array_element "day"))) (Utilities|Text|ToText(String) (Utilities|String|GetSubstring (.ReturnValue (Class|JsonFieldData|GetString _array_element "date")) 0 3)) (Utilities|Text|ToText(String) (Utilities|String|Append (Utilities|String|ToString(Integer) (Math|Float|Round (* (- (Math|Conversions|ToFloat(Integer) (.ReturnValue (Class|JsonFieldData|GetString _array_element "high"))) 32.0) (/ 5.0 9.0)))) "°")) _key)
            (elif (== _array_index 2)
              (bind _key_2 (CallFunction|DetermineWeatherIcon (Variables|Default|GetText)))
              (CallFunction|Day2 (Utilities|Text|ToText(String) (.ReturnValue (Class|JsonFieldData|GetString _array_element "day"))) (Utilities|Text|ToText(String) (Utilities|String|GetSubstring (.ReturnValue (Class|JsonFieldData|GetString _array_element "date")) 0 3)) (Utilities|Text|ToText(String) (Utilities|String|Append (Utilities|String|ToString(Integer) (Math|Float|Round (* (- (Math|Conversions|ToFloat(Integer) (.ReturnValue (Class|JsonFieldData|GetString _array_element "high"))) 32.0) (/ 5.0 9.0)))) "°")) _key_2)
              (elif (== _array_index 3)
                (bind _key_3 (CallFunction|DetermineWeatherIcon (Variables|Default|GetText)))
                (CallFunction|Day3 (Utilities|Text|ToText(String) (.ReturnValue (Class|JsonFieldData|GetString _array_element "day"))) (Utilities|Text|ToText(String) (Utilities|String|GetSubstring (.ReturnValue (Class|JsonFieldData|GetString _array_element "date")) 0 3)) (Utilities|Text|ToText(String) (Utilities|String|Append (Utilities|String|ToString(Integer) (Math|Float|Round (* (- (Math|Conversions|ToFloat(Integer) (.ReturnValue (Class|JsonFieldData|GetString _array_element "high"))) 32.0) (/ 5.0 9.0)))) "°")) _key_3)
                (elif (== _array_index 4)
                  (bind _key_4 (CallFunction|DetermineWeatherIcon (Variables|Default|GetText)))
                  (CallFunction|Day4 (Utilities|Text|ToText(String) (.ReturnValue (Class|JsonFieldData|GetString _array_element "day"))) (Utilities|Text|ToText(String) (Utilities|String|GetSubstring (.ReturnValue (Class|JsonFieldData|GetString _array_element "date")) 0 3)) (Utilities|Text|ToText(String) (Utilities|String|Append (Utilities|String|ToString(Integer) (Math|Float|Round (* (- (Math|Conversions|ToFloat(Integer) (.ReturnValue (Class|JsonFieldData|GetString _array_element "high"))) 32.0) (/ 5.0 9.0)))) "°")) _key_4)
                  (elif (== _array_index 5)
                    (bind _key_5 (CallFunction|DetermineWeatherIcon (Variables|Default|GetText)))
                    (CallFunction|Day5 (Utilities|Text|ToText(String) (.ReturnValue (Class|JsonFieldData|GetString _array_element "day"))) (Utilities|Text|ToText(String) (Utilities|String|GetSubstring (.ReturnValue (Class|JsonFieldData|GetString _array_element "date")) 0 3)) (Utilities|Text|ToText(String) (Utilities|String|Append (Utilities|String|ToString(Integer) (Math|Float|Round (* (- (Math|Conversions|ToFloat(Integer) (.ReturnValue (Class|JsonFieldData|GetString _array_element "high"))) 32.0) (/ 5.0 9.0)))) "°")) _key_5)))))))
        (else
          (Development|PrintString "Could not get forecast. Retrying")
          (CallFunction|GetWeatherAgain)))
      (else
        (Development|PrintString "Could not get object field")))
    (else
      (Development|PrintString "OnGetResult Failed"))))

(event Custom|Get%20Weather%20Again
  ;[1 1 1] Get weather information via JSON
  (bind _returnvalue (Class|JsonFieldData|GetRequest (Class|JsonFieldData|Create) (Variables|Default|GetURL)))
  (if (Utilities|IsValid _returnvalue)
    (EventDispatchers|AssignOnGetResult _returnvalue (delegate Custom|CustomEvent))
    (else
      (Development|PrintString "JSON Request Failed"))))

(event Collision|EventActorBeginOverlap
  (params (OtherActor :type Actor%20Object%20Reference)))

(event EventEndGrab
  (params (ReleasingController :type Motion%20Controller%20Component%20Object%20Reference) (AltButtonPressed :type Boolean) (Thrown :type Boolean))
  ;[1 1 1] Grab interface logic
  (if Thrown
    (Physics|SetSimulatePhysics (Variables|Default|GetCube) true)
    (Utilities|FlowControl|Delay 0.5)
    (Actor|DestroyActor)
    (else
      (Transformation|DetachFromActor "KeepWorld" "KeepWorld" "KeepWorld"))))

(event EventTick
  (params (DeltaSeconds :type Float%20%28single-precision%29))
  (if (Variables|Default|GetFirstTime)
    (Variables|Default|SetFirstTime false)
    (else
      (Utilities|FlowControl|Delay 1.8e+03)))
  ;[1 1 1] Get weather information via JSON
  (bind _returnvalue (Class|JsonFieldData|GetRequest (Class|JsonFieldData|Create) (Variables|Default|GetURL)))
  (if (Utilities|IsValid _returnvalue)
    (EventDispatchers|AssignOnGetResult _returnvalue (delegate Custom|CustomEvent))
    (else
      (Development|PrintString "JSON Request Failed"))))

(event EventStartGrab
  (params (GrabbingController :type Motion%20Controller%20Component%20Object%20Reference))
  ;[1 1 1] Grab interface logic
  (Transformation|AttachComponentToComponent (Variables|Default|GetDefaultSceneRoot) GrabbingController "None" "KeepWorld" "KeepWorld" "KeepWorld" true))

(fn ConstructionScript)

(fn Day1
  (params (Day :type Text) (Date :type Text) (Degree :type Text) (Key :type String))
  (bind _icon1 (Variables|Default|GetIcon1))
  (Rendering|Components|TextRender|SetText (Variables|Default|GetDay1) Day)
  (Rendering|Components|TextRender|SetText (Variables|Default|GetDate1) Date)
  (Rendering|Components|TextRender|SetText (Variables|Default|GetDegree1) Degree)
  (if (Utilities|Enum|Equal(Enum) Key "0")
    (Rendering|Material|SetMaterial _icon1 0 "/Game/VirtualOSContent/WeatherInformation/Materials/Lightning.Lightning")
    (elif (Utilities|Enum|Equal(Enum) Key "1")
      (Rendering|Material|SetMaterial _icon1 0 "/Game/VirtualOSContent/WeatherInformation/Materials/Rain.Rain")
      (elif (Utilities|Enum|Equal(Enum) Key "2")
        (Rendering|Material|SetMaterial _icon1 0 "/Game/VirtualOSContent/WeatherInformation/Materials/Cloud.Cloud")
        (elif (Utilities|Enum|Equal(Enum) Key "3")
          (Rendering|Material|SetMaterial _icon1 0 "/Game/VirtualOSContent/WeatherInformation/Materials/PartialCloud.PartialCloud")
          (elif (Utilities|Enum|Equal(Enum) Key "4")
            (Rendering|Material|SetMaterial _icon1 0 "/Game/VirtualOSContent/WeatherInformation/Materials/Sun.Sun")
            (elif (Utilities|Enum|Equal(Enum) Key "5")
              (Rendering|Material|SetMaterial _icon1 0 "/Game/VirtualOSContent/WeatherInformation/Materials/Snowing.Snowing"))))))))

(fn Day2
  (params (Day :type Text) (Date :type Text) (Degree :type Text) (Key :type String))
  (bind _icon2 (Variables|Default|GetIcon2))
  (Rendering|Components|TextRender|SetText (Variables|Default|GetDay2) Day)
  (Rendering|Components|TextRender|SetText (Variables|Default|GetDate2) Date)
  (Rendering|Components|TextRender|SetText (Variables|Default|GetDegree2) Degree)
  (if (Utilities|Enum|Equal(Enum) Key "0")
    (Rendering|Material|SetMaterial _icon2 0 "/Game/VirtualOSContent/WeatherInformation/Materials/Lightning.Lightning")
    (elif (Utilities|Enum|Equal(Enum) Key "1")
      (Rendering|Material|SetMaterial _icon2 0 "/Game/VirtualOSContent/WeatherInformation/Materials/Rain.Rain")
      (elif (Utilities|Enum|Equal(Enum) Key "2")
        (Rendering|Material|SetMaterial _icon2 0 "/Game/VirtualOSContent/WeatherInformation/Materials/Cloud.Cloud")
        (elif (Utilities|Enum|Equal(Enum) Key "3")
          (Rendering|Material|SetMaterial _icon2 0 "/Game/VirtualOSContent/WeatherInformation/Materials/PartialCloud.PartialCloud")
          (elif (Utilities|Enum|Equal(Enum) Key "4")
            (Rendering|Material|SetMaterial _icon2 0 "/Game/VirtualOSContent/WeatherInformation/Materials/Sun.Sun")
            (elif (Utilities|Enum|Equal(Enum) Key "5")
              (Rendering|Material|SetMaterial _icon2 0 "/Game/VirtualOSContent/WeatherInformation/Materials/Snowing.Snowing"))))))))

(fn Day3
  (params (Day :type Text) (Date :type Text) (Degree :type Text) (Key :type String))
  (bind _icon3 (Variables|Default|GetIcon3))
  (Rendering|Components|TextRender|SetText (Variables|Default|GetDay3) Day)
  (Rendering|Components|TextRender|SetText (Variables|Default|GetDate3) Date)
  (Rendering|Components|TextRender|SetText (Variables|Default|GetDegree3) Degree)
  (if (Utilities|Enum|Equal(Enum) Key "0")
    (Rendering|Material|SetMaterial _icon3 0 "/Game/VirtualOSContent/WeatherInformation/Materials/Lightning.Lightning")
    (elif (Utilities|Enum|Equal(Enum) Key "1")
      (Rendering|Material|SetMaterial _icon3 0 "/Game/VirtualOSContent/WeatherInformation/Materials/Rain.Rain")
      (elif (Utilities|Enum|Equal(Enum) Key "2")
        (Rendering|Material|SetMaterial _icon3 0 "/Game/VirtualOSContent/WeatherInformation/Materials/Cloud.Cloud")
        (elif (Utilities|Enum|Equal(Enum) Key "3")
          (Rendering|Material|SetMaterial _icon3 0 "/Game/VirtualOSContent/WeatherInformation/Materials/PartialCloud.PartialCloud")
          (elif (Utilities|Enum|Equal(Enum) Key "4")
            (Rendering|Material|SetMaterial _icon3 0 "/Game/VirtualOSContent/WeatherInformation/Materials/Sun.Sun")
            (elif (Utilities|Enum|Equal(Enum) Key "5")
              (Rendering|Material|SetMaterial _icon3 0 "/Game/VirtualOSContent/WeatherInformation/Materials/Snowing.Snowing"))))))))

(fn Day4
  (params (Day :type Text) (Date :type Text) (Degree :type Text) (Key :type String))
  (bind _icon4 (Variables|Default|GetIcon4))
  (Rendering|Components|TextRender|SetText (Variables|Default|GetDay4) Day)
  (Rendering|Components|TextRender|SetText (Variables|Default|GetDate4) Date)
  (Rendering|Components|TextRender|SetText (Variables|Default|GetDegree4) Degree)
  (if (Utilities|Enum|Equal(Enum) Key "0")
    (Rendering|Material|SetMaterial _icon4 0 "/Game/VirtualOSContent/WeatherInformation/Materials/Lightning.Lightning")
    (elif (Utilities|Enum|Equal(Enum) Key "1")
      (Rendering|Material|SetMaterial _icon4 0 "/Game/VirtualOSContent/WeatherInformation/Materials/Rain.Rain")
      (elif (Utilities|Enum|Equal(Enum) Key "2")
        (Rendering|Material|SetMaterial _icon4 0 "/Game/VirtualOSContent/WeatherInformation/Materials/Cloud.Cloud")
        (elif (Utilities|Enum|Equal(Enum) Key "3")
          (Rendering|Material|SetMaterial _icon4 0 "/Game/VirtualOSContent/WeatherInformation/Materials/PartialCloud.PartialCloud")
          (elif (Utilities|Enum|Equal(Enum) Key "4")
            (Rendering|Material|SetMaterial _icon4 0 "/Game/VirtualOSContent/WeatherInformation/Materials/Sun.Sun")
            (elif (Utilities|Enum|Equal(Enum) Key "5")
              (Rendering|Material|SetMaterial _icon4 0 "/Game/VirtualOSContent/WeatherInformation/Materials/Snowing.Snowing"))))))))

(fn Day5
  (params (Day :type Text) (Date :type Text) (Degree :type Text) (Key :type String))
  (bind _icon5 (Variables|Default|GetIcon5))
  (Rendering|Components|TextRender|SetText (Variables|Default|GetDay5) Day)
  (Rendering|Components|TextRender|SetText (Variables|Default|GetDate5) Date)
  (Rendering|Components|TextRender|SetText (Variables|Default|GetDegree5) Degree)
  (if (Utilities|Enum|Equal(Enum) Key "0")
    (Rendering|Material|SetMaterial _icon5 0 "/Game/VirtualOSContent/WeatherInformation/Materials/Lightning.Lightning")
    (elif (Utilities|Enum|Equal(Enum) Key "1")
      (Rendering|Material|SetMaterial _icon5 0 "/Game/VirtualOSContent/WeatherInformation/Materials/Rain.Rain")
      (elif (Utilities|Enum|Equal(Enum) Key "2")
        (Rendering|Material|SetMaterial _icon5 0 "/Game/VirtualOSContent/WeatherInformation/Materials/Cloud.Cloud")
        (elif (Utilities|Enum|Equal(Enum) Key "3")
          (Rendering|Material|SetMaterial _icon5 0 "/Game/VirtualOSContent/WeatherInformation/Materials/PartialCloud.PartialCloud")
          (elif (Utilities|Enum|Equal(Enum) Key "4")
            (Rendering|Material|SetMaterial _icon5 0 "/Game/VirtualOSContent/WeatherInformation/Materials/Sun.Sun")
            (elif (Utilities|Enum|Equal(Enum) Key "5")
              (Rendering|Material|SetMaterial _icon5 0 "/Game/VirtualOSContent/WeatherInformation/Materials/Snowing.Snowing"))))))))

(fn DetermineWeatherIcon
  (params (Text :type String))
  (for _array_element (Variables|Default|GetGroupLightning)
    (if (Utilities|Enum|Equal(Enum) _array_element Text)
      (return "0")))
  (for _array_element_2 (Variables|Default|GetGroupRain)
    (if (Utilities|Enum|Equal(Enum) _array_element_2 Text)
      (return "1")))
  (for _array_element_3 (Variables|Default|GetGroupCloud)
    (if (Utilities|Enum|Equal(Enum) _array_element_3 Text)
      (return "2")))
  (for _array_element_4 (Variables|Default|GetGroupPartlyCloudy)
    (if (Utilities|Enum|Equal(Enum) _array_element_4 Text)
      (return "3")))
  (for _array_element_5 (Variables|Default|GetGroupSun)
    (if (Utilities|Enum|Equal(Enum) _array_element_5 Text)
      (return "4")))
  (for _array_element_6 (Variables|Default|GetGroupSnow)
    (if (Utilities|Enum|Equal(Enum) Text _array_element_6)
      (return "5"))))

(fn GetProgramHologram
  (return "/Game/VirtualOSContent/WeatherInformation/iconSMWeather.iconSMWeather"))

(fn GetProgramName
  (return "Forecast"))

(fn IsRunning
  (return true))