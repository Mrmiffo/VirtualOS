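; Virtual OS menu actor with an HH:MM:SS clock and poke buttons that launch fake Spotify, Chrome and file browser apps.
; A first PokeSphere overlap starts the loading widget and records the logo's origin.
; Later overlaps nudge the logo along X until TestFunction's threshold, then light the button and spawn the app near the player.
; WristSphere overlaps destroy that app, restore the button and reset its flags after a delay.
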(event OnComponentBeginOverlap(FolderLogo)
  (params (OverlappedComponent :type Primitive%20Component%20Object%20Reference) (OtherActor :type Actor%20Object%20Reference) (OtherComp :type Primitive%20Component%20Object%20Reference) (OtherBodyIndex :type Integer) (bFromSweep :type Boolean) (SweepResult :type Hit%20Result%20Structure%20%28by%20ref%29))
  (bind _returnvalue (Game|Player|GetPlayerPawn 0))
  (bind _folderlogo (Variables|Default|GetFolderLogo))
  (bind _returnvalue_2 (Transformation|GetActorLocation _returnvalue))
  (bind _relativelocation (Variables|/Script/Engine.SceneComponent|GetRelativeLocation _folderlogo))
  (bind (_x _y _z) (Math|Vector|BreakVector _relativelocation))
  (bind (_x_2 _y_2 _z_2) (Math|Vector|BreakVector _returnvalue_2))
  ;[1 1 1] FileBrowserButton
  (if (Variables|Default|GetFileBrowserPendingKill)
    (Utilities|FlowControl|Delay 3.0)
    (Variables|Default|SetFileBrowserPendingKill false)
    (elif (Components|ComponentHasTag OtherComp "PokeSphere")
      (if (not (Variables|Default|GetFolderRunning))
        (if (Variables|Default|GetFolderSecondIterationOrMore)
          (if (Variables|Default|GetFolderIsDone)
            (Development|PrintString "Hello")
            (else
              (bind _newparam (CallFunction|TestFunction _relativelocation (Variables|Default|GetFolderOriginLocation)))
              (if _newparam
                (Transformation|SetRelativeLocation (Variables|Default|GetFolderLogo) (Math|Vector|MakeVector (+ _x -0.1) _y _z) false false)
                (else
                  (Rendering|Material|SetMaterial (Variables|Default|GetFolderLight) 0 "/Game/ClockRoom/BluePrints/DigitalClock/DigitalClockMaterials/BlackPolishedPlastic2Shine.BlackPolishedPlastic2Shine")
                  (bind _returnvalue_3 (Game|SpawnActorfromClass "/Game/VirtualOSContent/FileSystem/Blueprints/File_BP.File_BP_C" (Math|Transform|MakeTransform (Math|Vector|MakeVector (+ _x_2 1e+02) _y_2 _z_2) "0,180.000000, 0" "1.000000,1.000000,1.000000") "Undefined" 0 0))
                  (Variables|Default|SetFileBrowser _returnvalue_3)
                  (Development|PrintString "Spawn" true true "(R=0.000000,G=0.660000,B=1.000000,A=1.000000)" 1e+01)
                  (Variables|Default|SetFolderRunning true)
                  (Variables|Default|SetFolderIsDone true)
                  (Development|PrintString "ChromeRunning")))))
          (else
            (bind _asloading_gui (Utilities|Casting|CastToLoadingGUI (UserInterface|GetUserWidgetObject (Variables|Default|GetLoadingFile))))
            (Default|StartLoading _asloading_gui)
            (Utilities|FlowControl|Delay 2.0)
            (Variables|Default|SetFolderOriginLocation (Variables|/Script/Engine.SceneComponent|GetRelativeLocation (Variables|Default|GetFolderLogo)))
            (Variables|Default|SetFolderSecondIterationOrMore true))))
      (elif (Components|ComponentHasTag OtherComp "WristSphere")
        (CallFunction|CloseFileBrowser)
        (Variables|Default|SetFileBrowserPendingKill true)
        (Utilities|FlowControl|Delay 3.0)
        (CallFunction|FileBrowserBoolsFalse)))))

(event OnComponentBeginOverlap(SpotifyLogo)
  (params (OverlappedComponent :type Primitive%20Component%20Object%20Reference) (OtherActor :type Actor%20Object%20Reference) (OtherComp :type Primitive%20Component%20Object%20Reference) (OtherBodyIndex :type Integer) (bFromSweep :type Boolean) (SweepResult :type Hit%20Result%20Structure%20%28by%20ref%29))
  (bind _returnvalue (Game|Player|GetPlayerPawn 0))
  (bind _spotifylogo (Variables|Default|GetSpotifyLogo))
  (bind _returnvalue_2 (Transformation|GetActorLocation _returnvalue))
  (bind _relativelocation (Variables|/Script/Engine.SceneComponent|GetRelativeLocation _spotifylogo))
  (bind (_x _y _z) (Math|Vector|BreakVector _relativelocation))
  (bind (_x_2 _y_2 _z_2) (Math|Vector|BreakVector _returnvalue_2))
  ;[1 1 1] SpotifyButton
  (if (Variables|Default|GetSpotifyPendingKill)
    (Utilities|FlowControl|Delay 3.0)
    (Variables|Default|SetSpotifyPendingKill false)
    (elif (Components|ComponentHasTag OtherComp "PokeSphere")
      (if (not (Variables|Default|GetSpotifyRunning))
        (if (Variables|Default|GetSecondIterationOrMore)
          (if (Variables|Default|GetSpotifyIsDone)
            (Development|PrintString "Hello")
            (else
              (bind _newparam (CallFunction|TestFunction _relativelocation (Variables|Default|GetSpotifyOriginLocation)))
              (if _newparam
                (Transformation|SetRelativeLocation (Variables|Default|GetSpotifyLogo) (Math|Vector|MakeVector (+ _x -0.1) _y _z) false false)
                (else
                  (Rendering|Material|SetMaterial (Variables|Default|GetSpotifyLight) 0 "/Game/ClockRoom/BluePrints/DigitalClock/DigitalClockMaterials/BlackPolishedPlastic2Shine.BlackPolishedPlastic2Shine")
                  (bind _returnvalue_3 (Game|SpawnActorfromClass "/Game/SpawnRoom/WebBrowsers/SpotifyBrowser/SpotifyFakeBrowser/FakeSpotify_BP.FakeSpotify_BP_C" (Math|Transform|MakeTransform (Math|Vector|MakeVector (+ _x_2 1e+02) _y_2 _z_2) "0,180.000000, 0" "1.000000,1.000000,1.000000") "Undefined" 0 0))
                  (Variables|Default|SetFakeSpotify _returnvalue_3)
                  (Development|PrintString "Spawn" true true "(R=0.000000,G=0.660000,B=1.000000,A=1.000000)" 1e+01)
                  (Variables|Default|SetSpotifyRunning true)
                  (Variables|Default|SetSpotifyIsDone true)
                  (Development|PrintString "SpotifyRunning")))))
          (else
            (bind _asloading_gui (Utilities|Casting|CastToLoadingGUI (UserInterface|GetUserWidgetObject (Variables|Default|GetLoadingSpotify))))
            (Default|StartLoading _asloading_gui)
            (Utilities|FlowControl|Delay 2.0)
            (Variables|Default|SetSpotifyOriginLocation (Variables|/Script/Engine.SceneComponent|GetRelativeLocation (Variables|Default|GetSpotifyLogo)))
            (Variables|Default|SetSecondIterationOrMore true))))
      (elif (Components|ComponentHasTag OtherComp "WristSphere")
        (CallFunction|CloseSpotify)
        (Variables|Default|SetSpotifyPendingKill true)
        (Utilities|FlowControl|Delay 3.0)
        (CallFunction|SpotifyBoolsFalse)))))

(event OnComponentBeginOverlap(ChromeLogo)
  (params (OverlappedComponent :type Primitive%20Component%20Object%20Reference) (OtherActor :type Actor%20Object%20Reference) (OtherComp :type Primitive%20Component%20Object%20Reference) (OtherBodyIndex :type Integer) (bFromSweep :type Boolean) (SweepResult :type Hit%20Result%20Structure%20%28by%20ref%29))
  (bind _returnvalue (Game|Player|GetPlayerPawn 0))
  (bind _chromelogo (Variables|Default|GetChromeLogo))
  (bind _returnvalue_2 (Transformation|GetActorLocation _returnvalue))
  (bind _relativelocation (Variables|/Script/Engine.SceneComponent|GetRelativeLocation _chromelogo))
  (bind (_x _y _z) (Math|Vector|BreakVector _relativelocation))
  (bind (_x_2 _y_2 _z_2) (Math|Vector|BreakVector _returnvalue_2))
  ;[1 1 1] ChromeButton
  (if (Variables|Default|GetChromePendingKill)
    (Utilities|FlowControl|Delay 3.0)
    (Variables|Default|SetChromePendingKill false)
    (elif (Components|ComponentHasTag OtherComp "PokeSphere")
      (if (not (Variables|Default|GetChromeRunning))
        (if (Variables|Default|GetChromeSecondIterationOrMore)
          (if (Variables|Default|GetChromeIsDone)
            (Development|PrintString "Hello")
            (else
              (bind _newparam (CallFunction|TestFunction _relativelocation (Variables|Default|GetChromeOriginLocation)))
              (if _newparam
                (Transformation|SetRelativeLocation (Variables|Default|GetChromeLogo) (Math|Vector|MakeVector (+ _x -0.1) _y _z) false false)
                (else
                  (Rendering|Material|SetMaterial (Variables|Default|GetChromeLight) 0 "/Game/ClockRoom/BluePrints/DigitalClock/DigitalClockMaterials/BlackPolishedPlastic2Shine.BlackPolishedPlastic2Shine")
                  (bind _returnvalue_3 (Game|SpawnActorfromClass "/Game/SpawnRoom/WebBrowsers/ChromeBrowser/ChromeBrowser_BP.ChromeBrowser_BP_C" (Math|Transform|MakeTransform (Math|Vector|MakeVector (+ _x_2 1e+02) _y_2 _z_2) "0,180.000000, 0" "1.000000,1.000000,1.000000") "Undefined" 0 0))
                  (Variables|Default|SetChrome _returnvalue_3)
                  (Development|PrintString "Spawn" true true "(R=0.000000,G=0.660000,B=1.000000,A=1.000000)" 1e+01)
                  (Variables|Default|SetChromeRunning true)
                  (Variables|Default|SetChromeIsDone true)
                  (Development|PrintString "ChromeRunning")))))
          (else
            (bind _asloading_gui (Utilities|Casting|CastToLoadingGUI (UserInterface|GetUserWidgetObject (Variables|Default|GetLoadingChrome))))
            (Default|StartLoading _asloading_gui)
            (Utilities|FlowControl|Delay 2.0)
            (Variables|Default|SetChromeOriginLocation (Variables|/Script/Engine.SceneComponent|GetRelativeLocation (Variables|Default|GetChromeLogo)))
            (Variables|Default|SetChromeSecondIterationOrMore true))))
      (elif (Components|ComponentHasTag OtherComp "WristSphere")
        (CallFunction|CloseChrome)
        (Variables|Default|SetChromePendingKill true)
        (Utilities|FlowControl|Delay 0.2)
        (CallFunction|ChromeBoolsFalse)))))

(event EventBeginPlay)

(event Collision|EventActorBeginOverlap
  (params (OtherActor :type Actor%20Object%20Reference)))

(event EventTick
  (params (DeltaSeconds :type Float%20%28single-precision%29))
  (bind _returnvalue (Math|DateTime|Now))
  (bind _returnvalue_2 (Class|KismetMathLibrary|GetHour _returnvalue))
  (bind _returnvalue_3 (Class|KismetMathLibrary|GetMinute _returnvalue))
  (bind _returnvalue_4 (Class|KismetMathLibrary|GetSecond _returnvalue))
  (bind _returnvalue_5 (Utilities|String|ToString(Integer) _returnvalue_2))
  (bind _returnvalue_6 (Utilities|String|ToString(Integer) _returnvalue_3))
  (bind _returnvalue_7 (Utilities|String|ToString(Integer) _returnvalue_4))
  ;[1 1 1] Digital clock with format 00:00:00
  (Rendering|Components|TextRender|SetText (Variables|Default|GetDigits) (Utilities|Text|ToText(String) (Utilities|String|Append (select (> _returnvalue_2 9) _returnvalue_5 (Utilities|String|Append "0" _returnvalue_5)) ":" (select (> _returnvalue_3 9) _returnvalue_6 (Utilities|String|Append "0" _returnvalue_6)) ":" (select (> _returnvalue_4 9) _returnvalue_7 (Utilities|String|Append "0" _returnvalue_7))))))

(fn ConstructionScript)

(fn TestFunction
  (params (CurrentPos :type Vector) (OriginPos :type Vector))
  (if (<= (- (.X (Math|Vector|BreakVector OriginPos)) (.X (Math|Vector|BreakVector CurrentPos))) 1.0)
    (LocalVariables|SetLocalDone true)
    (else
      (LocalVariables|SetLocalDone false)))
  (return (LocalVariables|GetLocalDone)))

(fn CloseChrome
  (if (Variables|Default|GetChromeRunning)
    (Actor|DestroyActor (Variables|Default|GetChrome))
    (Rendering|Material|SetMaterial (Variables|Default|GetChromeLight) 0 "/Game/ClockRoom/BluePrints/DigitalClock/DigitalClockMaterials/BlackPolishedPlastic.BlackPolishedPlastic")
    (Transformation|SetRelativeLocation (Variables|Default|GetChromeLogo) (Variables|Default|GetChromeOriginLocation) false false)))

(fn CloseSpotify
  (if (Variables|Default|GetSpotifyRunning)
    (Actor|DestroyActor (Variables|Default|GetFakeSpotify))
    (Rendering|Material|SetMaterial (Variables|Default|GetSpotifyLight) 0 "/Game/ClockRoom/BluePrints/DigitalClock/DigitalClockMaterials/BlackPolishedPlastic.BlackPolishedPlastic")
    (Transformation|SetRelativeLocation (Variables|Default|GetSpotifyLogo) (Variables|Default|GetSpotifyOriginLocation) false false)))

(fn CloseFileBrowser
  (if (Variables|Default|GetFolderRunning)
    (Actor|DestroyActor (Variables|Default|GetFileBrowser))
    (Rendering|Material|SetMaterial (Variables|Default|GetFolderLight) 0 "/Game/ClockRoom/BluePrints/DigitalClock/DigitalClockMaterials/BlackPolishedPlastic.BlackPolishedPlastic")
    (Transformation|SetRelativeLocation (Variables|Default|GetFolderLogo) (Variables|Default|GetFolderOriginLocation) false false)))

(fn SpotifyBoolsFalse
  (Variables|Default|SetSpotifyRunning false)
  (Variables|Default|SetSpotifyIsDone false)
  (Variables|Default|SetSecondIterationOrMore false))

(fn ChromeBoolsFalse
  (Variables|Default|SetChromeRunning false)
  (Variables|Default|SetChromeIsDone false)
  (Variables|Default|SetChromeSecondIterationOrMore false))

(fn FileBrowserBoolsFalse
  (Variables|Default|SetFolderRunning false)
  (Variables|Default|SetFolderIsDone false)
  (Variables|Default|SetFolderSecondIterationOrMore false))

(fn NewFunction0
  (bind _asloading_gui (Utilities|Casting|CastToLoadingGUI (UserInterface|GetUserWidgetObject (Variables|Default|GetLoadingSpotify))))
  (Default|StartLoading _asloading_gui))