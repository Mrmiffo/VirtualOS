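; Grabbable keyboard actor that hosts a KeyBoard_WB_old widget for text input.
; On BeginPlay it hands its WidgetInteraction to the widget and binds the send press to an empty handler; the target display's goal-text check is disconnected debug code.
; Grabbing attaches it to the controller; the same controller's release detaches it, or on a throw enables Cube physics and destroys the actor after a short delay.
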(event Custom|SendPressed_Event_0
  ;[1 1 1] Getting keyboard inputs and outputs it on the display.
)

(event EventBeginPlay
  ;[1 1 1] Getting keyboard inputs and outputs it on the display.
  (bind _askey_board_wb_old (Utilities|Casting|CastToKeyBoard_WB_old (UserInterface|GetUserWidgetObject (Variables|Default|GetWidget))))
  (Variables|/Game/SpawnRoom/KeyBoard/Widgets/KeyBoard_WB_old.KeyBoard_WB_old_C|SetWidgetInteraction _askey_board_wb_old (Variables|Default|GetWidgetInteraction))
  (Development|PrintString "i keyboard bp")
  (EventDispatchers|AssignSendPressed _askey_board_wb_old (delegate Custom|SendPressed_Event_0)))

(event Collision|EventActorBeginOverlap
  (params (OtherActor :type Actor%20Object%20Reference)))

(event EventStartGrab
  (params (GrabbingController :type Motion%20Controller%20Component%20Object%20Reference))
  ;[1 1 1] Grab and release
  (bind _output_get (Variables|Default|SetGrabbingController GrabbingController))
  (Transformation|AttachComponentToComponent (Variables|Default|GetDefaultSceneRoot) _output_get "None" "KeepWorld" "KeepWorld" "KeepWorld" true))

(event EventTick
  (params (DeltaSeconds :type Float%20%28single-precision%29)))

(event EventEndGrab
  (params (ReleasingController :type Motion%20Controller%20Component%20Object%20Reference) (AltButtonPressed :type Boolean) (Thrown :type Boolean))
  ;[1 1 1] Grab and release
  (if (== ReleasingController (Variables|Default|GetGrabbingController))
    (if Thrown
      (Physics|SetSimulatePhysics (Variables|Default|GetCube) true)
      (Utilities|FlowControl|Delay 2.0)
      (Actor|DestroyActor)
      (else
        (Transformation|DetachFromActor "KeepWorld" "KeepWorld" "KeepWorld")))))

(fn ConstructionScript)