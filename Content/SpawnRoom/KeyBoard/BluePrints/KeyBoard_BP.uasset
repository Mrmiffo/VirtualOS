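; KeyBoard_BP is a keyboard actor whose widget component hosts a KeyBoard_WB, apparently for typing into a separate display.
; On BeginPlay it passes its WidgetInteraction to that widget, prints a debug string and binds to the widget's SendPressed event.
; The SendPressed handler is empty.
; A disconnected debug branch would compare TargetDisplay's KeyboardDisplay_WB text with GoalText and print whether it is correct.
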(event Custom|SendPressed_Event_0
  ;[1 1 1] Getting keyboard inputs and outputs it on the display.
)

(event EventBeginPlay
  ;[1 1 1] Getting keyboard inputs and outputs it on the display.
  (bind _askey_board_wb (Utilities|Casting|CastToKeyBoard_WB (UserInterface|GetUserWidgetObject (Variables|Default|GetWidget))))
  (Variables|/Game/SpawnRoom/KeyBoard/Widgets/KeyBoard_WB.KeyBoard_WB_C|SetWidgetInteraction _askey_board_wb (Variables|Default|GetWidgetInteraction))
  (Development|PrintString "i keyboard bp")
  (EventDispatchers|AssignSendPressed _askey_board_wb (delegate Custom|SendPressed_Event_0)))

(event Collision|EventActorBeginOverlap
  (params (OtherActor :type Actor%20Object%20Reference)))

(event EventTick
  (params (DeltaSeconds :type Float%20%28single-precision%29)))

(fn ConstructionScript)