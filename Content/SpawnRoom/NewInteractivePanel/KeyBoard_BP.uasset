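; Interactive keyboard actor in the spawn room panel that submits text entered on a linked display.
; On BeginPlay it passes its WidgetInteraction to the KeyBoard_WB widget and binds that widget's SendPressed event.
; On send, it reads the text box in TargetDisplay's KeyboardDisplay_WB widget and compares it to GoalText.
; The result is only a debug print of correct or not correct, standing in for a real action.
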(event Custom|SendPressed_Event_0
  ;[1 1 1] Getting keyboard inputs and outputs it on the display.
  (bind _askeyboard_display_wb (Utilities|Casting|CastToKeyboardDisplay_WB (UserInterface|GetUserWidgetObject (Variables|/Game/SpawnRoom/NewInteractivePanel/KeyBoardDisplay_BP.KeyBoardDisplay_BP_C|GetWidget (Variables|Default|GetTargetDisplay)))))
  ;;[1 1 1] Debugging. Instead of this -> Do the action one want, e.g. search file etc...
  (if (Utilities|Enum|Equal(Enum) (Class|EditableTextBox|GetText (Variables|/Game/SpawnRoom/NewInteractivePanel/KeyboardDisplay_WB.KeyboardDisplay_WB_C|GetEditableTextBox_0 _askeyboard_display_wb)) (Variables|Default|GetGoalText))
    (Development|PrintString "Correct!")
    (else
      (Development|PrintString "Not Correct!"))))

(event EventBeginPlay
  ;[1 1 1] Getting keyboard inputs and outputs it on the display.
  (bind _askey_board_wb (Utilities|Casting|CastToKeyBoard_WB (UserInterface|GetUserWidgetObject (Variables|Default|GetWidget))))
  (Variables|/Game/SpawnRoom/NewInteractivePanel/KeyBoard_WB.KeyBoard_WB_C|SetWidgetInteraction _askey_board_wb (Variables|Default|GetWidgetInteraction))
  (EventDispatchers|AssignSendPressed _askey_board_wb (delegate Custom|SendPressed_Event_0)))

(event Collision|EventActorBeginOverlap
  (params (OtherActor :type Actor%20Object%20Reference)))

(event EventTick
  (params (DeltaSeconds :type Float%20%28single-precision%29)))

(fn ConstructionScript)